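; Master VR weapon Blueprint that registers itself on the pawn when gripped and handles firing, ammo and reload.
; Construction copies WeaponValues into variables, scaling damage and magazine size by rarity.
; Tick traces from the muzzle to place an aim widget facing the pawn.
; Shot loops on a cooldown for automatics or fires once, playing only VFX and sound; overlapping ammo on RechargeTrigger refills, blocking new shots during a delay.
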(event OnComponentBeginOverlap(RechargeTrigger)
  (params (OverlappedComponent :type Primitive%20Component%20Object%20Reference) (OtherActor :type Actor%20Object%20Reference) (OtherComp :type Primitive%20Component%20Object%20Reference) (OtherBodyIndex :type Integer) (bFromSweep :type Boolean) (SweepResult :type Hit%20Result%20Structure%20%28by%20ref%29))
  ;[1 0 0.0312] RELOAD WEAPON
  (Utilities|Casting|CastToBP_GO_Municion OtherActor)
  (CallFunction|Reload))

(event Custom|Reload
  (bind _weapon_values_bullets_amount (Variables|Default|GetWeapon%20Values%20Bullets%20Amount))
  ;[1 0 0.0312] RELOAD WEAPON
  (if (< (Variables|Default|GetWeapon%20Values%20Bullets%20Left) _weapon_values_bullets_amount)
    (Variables|Default|SetisReloading true)
    (Variables|Default|SetWeapon%20Values%20Bullets%20Left _weapon_values_bullets_amount)
    (Utilities|FlowControl|Delay (Variables|Default|GetReloadTime))
    (Variables|Default|SetisReloading false)
    (else
      (Development|PrintString "Municion Llena"))))

(event Custom|Shot
  (params (isShooting :type Boolean))
  ;[0.5482 0 1] SHOT INPUT, SFX & VFX
  (if (and isShooting (not (Variables|Default|GetisReloading)))
    (if (and (Variables|Default|GetWeapon%20Values%20Automatic%20Weapon) isShooting)
      (if (and isShooting (> (Variables|Default|GetWeapon%20Values%20Bullets%20Left) 0.0)) :!label _label
        (Math|Float|DecrementFloat (Variables|Default|GetWeapon%20Values%20Bullets%20Left)
          (:%20%20
            (CallFunction|ShotWeapon)
            (Utilities|FlowControl|Delay (Variables|Default|GetWeapon%20Values%20Shot%20Cooldown))
            (goto _label))))
      (elif (> (Variables|Default|GetWeapon%20Values%20Bullets%20Left) 0.0)
        (Math|Float|DecrementFloat (Variables|Default|GetWeapon%20Values%20Bullets%20Left)
          (:%20%20
            (CallFunction|ShotWeapon)))
        (else
          (Development|PrintString "BP_MASTERWEAPON: NO BULLETS FEEDBACK"))))
    (else
      (CallFunction|ResetShot))))

(event Custom|ShootCheck
  (bind _as_vrpawn (Variables|Default|GetAs%20VRPawn))
  (bind _shotpoint (Variables|Default|GetShotPoint))
  (bind _shotobjective (Variables|Default|GetShotObjective))
  (bind _returnvalue (Transformation|GetWorldLocation _shotobjective))
  (bind _returnvalue_2 (Transformation|GetWorldLocation _shotpoint))
  (bind _rootcomponent (Variables|/Script/Engine.Actor|GetRootComponent _as_vrpawn))
  (bind _returnvalue_3 (Transformation|GetWorldLocation _rootcomponent))
  (bind _returnvalue_4 (Math|Rotator|FindLookatRotation _returnvalue _returnvalue_3))
  ;[0.001249 0.001937 1] SET SHOT OBJECTIVE WIDGET FACED CAMERA AND LINE TRACE SHOOT
  (bind _outhit (Collision|LineTraceByChannel _returnvalue_2 (* (* _returnvalue_2 (Math|Vector|GetForwardVector _shotpoint)) 5.0) "TraceTypeQuery2" false 0 "None"))
  (if (.bblockinghit _outhit)
    (Transformation|SetWorldLocationAndRotation _shotobjective (.location _outhit) _returnvalue_4 false false)
    (Variables|Default|SetOut%20Hit%20Location (.location _outhit))
    (else
      (Transformation|SetWorldLocationAndRotation _shotobjective (.traceend _outhit) _returnvalue_4 false false))))

(event Custom|ShotWeapon
  ;[0.5482 0 1] SHOT INPUT, SFX & VFX
  (Effects|SpawnEmitteratLocation (Variables|Default|GetWeapon%20Values%20Shot%20Fire%20VFX) (Transformation|GetWorldLocation (Variables|Default|GetShotPoint)))
  (Audio|PlaySoundatLocation (Variables|Default|GetWeapon%20Values%20Shot%20Fire%20SFX) (Transformation|GetWorldLocation (Variables|Default|GetStaticMeshComponent)) "0, 0, 0" 1.0 1.0 0.0 0 0 0 0))

(event Custom|ResetShot
  ;[0.5482 0 1] SHOT INPUT, SFX & VFX
)

(event EventTick
  (params (DeltaSeconds :type Float%20%28single-precision%29))
  (CallFunction|ShootCheck))

(event EventBeginPlay
  (bind _returnvalue (Actor|GetActorOfClass "/Game/VRTemplate/Blueprints/VRPawn.VRPawn_C"))
  (Variables|Default|SetAs%20VRPawn _returnvalue))

(event EventOnGrip
  (params (GrippingController :type Grip%20Motion%20Controller%20Component%20Object%20Reference) (GripInformation :type BP%20Actor%20Grip%20Information%20Structure%20%28by%20ref%29))
  ;[1 0.8816 0] GRIP
  (Development|PrintString (Utilities|String|ToString(Name) (Variables|/Script/HeadMountedDisplay.MotionControllerComponent|GetMotionSource GrippingController)))
  (Variables|/Game/VRTemplate/Blueprints/VRPawn.VRPawn_C|SetWeapon (Variables|Default|GetAs%20VRPawn) self))

(fn ConstructionScript
  (bind _weapon_values (Variables|Default|GetWeapon%20Values))
  (Variables|Default|SetWeapon%20Values%20Damage (* (.damage _weapon_values) (Utilities|Select :Index (.weaponrarity _weapon_values) :Option%200 0.0 :Option%201 0.0 :Option%202 0.0 :Option%203 0.0)))
  (Variables|Default|SetWeapon%20Values%20Shot%20Cooldown (.shotcooldown _weapon_values))
  (bind _output_get (Variables|Default|SetWeapon%20Values%20Bullets%20Amount (* (.bulletsamount _weapon_values) (Utilities|Select :Index (.weaponrarity _weapon_values) :Option%200 0.0 :Option%201 0.0 :Option%202 0.0 :Option%203 0.0))))
  (Variables|Default|SetWeapon%20Values%20Bullets%20Left _output_get)
  (Variables|Default|SetWeapon%20Values%20Automatic%20Weapon (.automaticweapon _weapon_values))
  (Variables|Default|SetWeapon%20Values%20Shot%20Fire%20VFX (.shotfirevfx _weapon_values))
  (Variables|Default|SetWeapon%20Values%20Shot%20Fire%20SFX (.shotfiresfx _weapon_values)))