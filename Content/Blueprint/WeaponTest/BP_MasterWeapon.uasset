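; Master weapon Blueprint that attaches to the player's WeaponPoint on grip overlap and handles aiming, firing and reloading.
; The construction script derives stats from WeaponValues, scaling damage and magazine size by rarity.
; Tick runs a line trace from ShotPoint to place an aim marker turned toward the player.
; Shot supports automatic or single fire with only VFX and sound, no damage applied; overlapping BP_PM_Municion triggers a timed reload.
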(event OnComponentBeginOverlap(RechargeTrigger)
  (params (OverlappedComponent :type Primitive%20Component%20Object%20Reference) (OtherActor :type Actor%20Object%20Reference) (OtherComp :type Primitive%20Component%20Object%20Reference) (OtherBodyIndex :type Integer) (bFromSweep :type Boolean) (SweepResult :type Hit%20Result%20Structure%20%28by%20ref%29))
  ;[1 0 0.0312] RELOAD WEAPON
  (Utilities|Casting|CastToBP_PM_Municion OtherActor)
  (CallFunction|Reload))

(event OnComponentBeginOverlap(GripTrigger)
  (params (OverlappedComponent :type Primitive%20Component%20Object%20Reference) (OtherActor :type Actor%20Object%20Reference) (OtherComp :type Primitive%20Component%20Object%20Reference) (OtherBodyIndex :type Integer) (bFromSweep :type Boolean) (SweepResult :type Hit%20Result%20Structure%20%28by%20ref%29))
  ;[0.01121 1 0] DEBUG - BORRAR
  (bind _asbp_third_person_character (Utilities|Casting|CastToBP_ThirdPersonCharacter OtherActor))
  (Variables|Default|SetBP_Player%20REF _asbp_third_person_character)
  (Variables|/Game/ThirdPerson/Blueprints/BP_ThirdPersonCharacter.BP_ThirdPersonCharacter_C|SetWeapon _asbp_third_person_character self)
  (Transformation|SetActorLocation (Transformation|GetWorldLocation (Variables|/Game/ThirdPerson/Blueprints/BP_ThirdPersonCharacter.BP_ThirdPersonCharacter_C|GetWeaponPoint (Variables|Default|GetBP_Player%20REF))) false true)
  (Transformation|AttachComponentToComponent (Variables|/Game/ThirdPerson/Blueprints/BP_ThirdPersonCharacter.BP_ThirdPersonCharacter_C|GetWeaponPoint (Variables|Default|GetBP_Player%20REF)) "None" "KeepRelative" "KeepRelative" "KeepRelative" true))

(event Custom|Reload
  (bind _weapon_values_bullets_amount (Variables|Default|GetWeapon%20Values%20Bullets%20Amount))
  ;[1 0 0.0312] RELOAD WEAPON
  (if (< (Variables|Default|GetWeapon%20Values%20Bullets%20Left) _weapon_values_bullets_amount)
    (Variables|Default|SetisReloading true)
    (Variables|Default|SetWeapon%20Values%20Bullets%20Left _weapon_values_bullets_amount)
    (Utilities|FlowControl|Delay (Variables|Default|GetReloadTime))
    (Variables|Default|SetisReloading false)
    (else
      (Development|PrintString "Municion Llena"))))

(event Custom|Shot
  (bind _bp_player_ref (Variables|Default|GetBP_Player%20REF))
  (bind _isshooting (Variables|/Game/ThirdPerson/Blueprints/BP_ThirdPersonCharacter.BP_ThirdPersonCharacter_C|GetisShooting _bp_player_ref))
  ;[0.5482 0 1] SHOT INPUT, SFX & VFX
  (if (and _isshooting (not (Variables|Default|GetisReloading)))
    (if (and (Variables|Default|GetWeapon%20Values%20Automatic%20Weapon) _isshooting)
      (if (and _isshooting (> (Variables|Default|GetWeapon%20Values%20Bullets%20Left) 0.0)) :!label _label
        (Math|Float|DecrementFloat (Variables|Default|GetWeapon%20Values%20Bullets%20Left)
          (:%20%20
            (CallFunction|ShotWeapon)
            (Utilities|FlowControl|Delay (Variables|Default|GetWeapon%20Values%20Shot%20Cooldown))
            (goto _label))))
      (elif (> (Variables|Default|GetWeapon%20Values%20Bullets%20Left) 0.0)
        (Math|Float|DecrementFloat (Variables|Default|GetWeapon%20Values%20Bullets%20Left)
          (:%20%20
            (CallFunction|ShotWeapon)))
        (else
          (Development|PrintString "BP_MASTERWEAPON: NO BULLETS FEEDBACK"))))
    (else
      (CallFunction|ResetShot))))

(event Custom|ShootCheck
  (bind _shotpoint (Variables|Default|GetShotPoint))
  (bind _shotobjective (Variables|Default|GetShotObjective))
  (bind _bp_player_ref (Variables|Default|GetBP_Player%20REF))
  (bind _returnvalue (Transformation|GetWorldLocation _shotobjective))
  (bind _returnvalue_2 (Transformation|GetWorldLocation _shotpoint))
  (bind _capsulecomponent (Variables|/Script/Engine.Character|GetCapsuleComponent _bp_player_ref))
  (bind _returnvalue_3 (Transformation|GetWorldLocation _capsulecomponent))
  (bind _returnvalue_4 (Math|Rotator|FindLookatRotation _returnvalue _returnvalue_3))
  ;[0.001249 0.001937 1] SET SHOT OBJECTIVE WIDGET FACED CAMERA AND LINE TRACE SHOOT
  (bind _outhit (Collision|LineTraceByChannel _returnvalue_2 (* (* _returnvalue_2 (Math|Vector|GetForwardVector _shotpoint)) 5.0) "TraceTypeQuery2" false 0 "None"))
  (if (.bblockinghit _outhit)
    (Transformation|SetWorldLocationAndRotation _shotobjective (.location _outhit) _returnvalue_4 false false)
    (Variables|Default|SetOut%20Hit%20Location (.location _outhit))
    (else
      (Transformation|SetWorldLocationAndRotation _shotobjective (.traceend _outhit) _returnvalue_4 false false))))

(event Custom|ShotWeapon
  ;[0.5482 0 1] SHOT INPUT, SFX & VFX
  (Effects|SpawnEmitteratLocation (Variables|Default|GetWeapon%20Values%20Shot%20Fire%20VFX) (Transformation|GetWorldLocation (Variables|Default|GetShotPoint)))
  (Audio|PlaySoundatLocation (Variables|Default|GetWeapon%20Values%20Shot%20Fire%20SFX) (Transformation|GetWorldLocation (Variables|Debug|GetStaticMeshComponent)) "0, 0, 0" 1.0 1.0 0.0 0 0 0 0))

(event Custom|ResetShot
  ;[0.5482 0 1] SHOT INPUT, SFX & VFX
)

(event EventTick
  (params (DeltaSeconds :type Float%20%28single-precision%29))
  (CallFunction|ShootCheck))

(event EventBeginPlay
  (bind _returnvalue (Actor|GetActorOfClass "/Game/ThirdPerson/Blueprints/BP_ThirdPersonCharacter.BP_ThirdPersonCharacter_C"))
  (Variables|Default|SetBP_Player%20REF _returnvalue))

(fn ConstructionScript
  (bind _weapon_values (Variables|Default|GetWeapon%20Values))
  (Variables|Default|SetWeapon%20Values%20Damage (* (.damage _weapon_values) (Utilities|Select :Index (.weaponrarity _weapon_values) :NewEnumerator0 1.0 :NewEnumerator1 1.25 :NewEnumerator2 1.5 :NewEnumerator3 2.0)))
  (Variables|Default|SetWeapon%20Values%20Shot%20Cooldown (.shotcooldown _weapon_values))
  (bind _output_get (Variables|Default|SetWeapon%20Values%20Bullets%20Amount (* (.bulletsamount _weapon_values) (Utilities|Select :Index (.weaponrarity _weapon_values) :NewEnumerator0 1.0 :NewEnumerator1 0.9 :NewEnumerator2 0.8 :NewEnumerator3 0.7))))
  (Variables|Default|SetWeapon%20Values%20Bullets%20Left _output_get)
  (Variables|Default|SetWeapon%20Values%20Automatic%20Weapon (.automaticweapon _weapon_values))
  (Variables|Default|SetWeapon%20Values%20Shot%20Fire%20VFX (.shotfirevfx _weapon_values))
  (Variables|Default|SetWeapon%20Values%20Shot%20Fire%20SFX (.shotfiresfx _weapon_values)))