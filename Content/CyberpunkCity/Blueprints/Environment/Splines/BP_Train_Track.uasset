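; Spline train track actor that shuttles a train back and forth along its spline when TrainFunctional is set.
; The construction script spawns carts cycling through CartMeshes and previews them at TrainPosition.
; At BeginPlay, the TrainMovement timeline runs at TrainSpeed, reversing after each TrainWaitingTime pause.
; MoveTrain spaces carts, Front and 180-degree-flipped Back along the spline by CartSpacing, with a TrainDeviation height offset.
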(event EventBeginPlay
  (if (Variables|Default|GetTrainFunctional)
    ;[1 1 1] Train Speed
    (Components|Timeline|SetPlayRate (Variables|Default|GetTrainMovement) (Variables|Default|GetTrainSpeed))
    ;[1 1 1] Train Movement Logic
    (if (Utilities|Enum|Equal(Enum) (stale _direction) "Forward") :!label _label
      (bind (_direction _trainposition) (Timeline|TrainMovement ReverseFromEnd)
        (:Update
          (CallFunction|MoveTrain _trainposition))
        (:Finished
          (Utilities|FlowControl|Delay (Variables|Default|GetTrainWaitingTime))
          (goto _label)))
      (else
        (Timeline|TrainMovement PlayFromStart)))))

(event Collision|EventActorBeginOverlap
  (params (OtherActor :type Actor%20Object%20Reference)))

(event EventTick
  (params (DeltaSeconds :type Float%20%28single-precision%29)))

(fn ConstructionScript
  (|CallParentFunction)
  (CallFunction|CreateTrain)
  (CallFunction|MoveTrain (Variables|Default|GetTrainPosition)))

(fn MoveTrain
  (params (TrainPosition :type Float%20%28double-precision%29))
  (bind _cartspacing (Variables|Default|GetCartSpacing))
  (bind _spline (Variables|Default|GetSpline))
  (bind _cartspacing_2 (Variables|Default|GetCartSpacing))
  (bind _traincarts (Variables|Default|GetTrainCarts))
  (bind _numberofcarts (Variables|Default|GetNumberOfCarts))
  (bind _cartspacing_3 (Variables|Default|GetCartSpacing))
  (bind _spline_2 (Variables|Default|GetSpline))
  (bind _spline_3 (Variables|Default|GetSpline))
  (bind _returnvalue (Utilities|Array|Length _traincarts))
  (bind _returnvalue_2 (Spline|GetSplineLength _spline_3))
  (bind _returnvalue_3 (* 1 _cartspacing))
  (bind _returnvalue_4 (* 2 _cartspacing_3))
  (bind _returnvalue_5 (+ _numberofcarts 2))
  (bind _returnvalue_6 (* _returnvalue_5 _cartspacing_3))
  (bind _returnvalue_7 (* _returnvalue_4 -1.0))
  (bind _returnvalue_8 (+ _returnvalue 2))
  (bind _returnvalue_9 (* _returnvalue_8 _cartspacing_2))
  (bind _returnvalue_10 (- _returnvalue_2 _returnvalue_6))
  (bind _returnvalue_11 (Math|Float|Lerp _returnvalue_7 _returnvalue_10 TrainPosition))
  (bind _returnvalue_12 (+ _returnvalue_11 _returnvalue_3))
  (bind _returnvalue_13 (+ _returnvalue_11 _returnvalue_9))
  (bind _returnvalue_14 (Spline|GetLocationatDistanceAlongSpline _spline_2 _returnvalue_12 "Local"))
  (bind _returnvalue_15 (Spline|GetRotationatDistanceAlongSpline _spline_2 _returnvalue_12 "Local"))
  (bind _returnvalue_16 (Spline|GetLocationatDistanceAlongSpline _spline _returnvalue_13 "Local"))
  (bind _returnvalue_17 (Spline|GetRotationatDistanceAlongSpline _spline _returnvalue_13 "Local"))
  (bind (_roll _pitch _yaw) (Math|Rotator|BreakRotator _returnvalue_15))
  (bind (_roll_2 _pitch_2 _yaw_2) (Math|Rotator|BreakRotator _returnvalue_17))
  (bind (_x _y _z) (Math|Vector|BreakVector _returnvalue_16))
  (bind (_x_2 _y_2 _z_2) (Math|Vector|BreakVector _returnvalue_14))
  ;[1 1 1] Move Carts
  (for (_array_element _array_index) (Variables|Default|GetTrainCarts)
    (Transformation|SetRelativeLocationAndRotation _array_element (Math|Vector|MakeVector (.X (Math|Vector|BreakVector (Spline|GetLocationatDistanceAlongSpline _spline_3 (+ _returnvalue_11 (* (+ _array_index 2) (Variables|Default|GetCartSpacing))) "Local"))) (.Y (Math|Vector|BreakVector (Spline|GetLocationatDistanceAlongSpline _spline_3 (+ _returnvalue_11 (* (+ _array_index 2) (Variables|Default|GetCartSpacing))) "Local"))) (+ (.Z (Math|Vector|BreakVector (Spline|GetLocationatDistanceAlongSpline _spline_3 (+ _returnvalue_11 (* (+ _array_index 2) (Variables|Default|GetCartSpacing))) "Local"))) (Variables|Default|GetTrainDeviation))) (Math|Rotator|MakeRotator (.Roll (Math|Rotator|BreakRotator (Spline|GetRotationatDistanceAlongSpline _spline_3 (+ _returnvalue_11 (* (+ _array_index 2) (Variables|Default|GetCartSpacing))) "Local"))) (.Pitch (Math|Rotator|BreakRotator (Spline|GetRotationatDistanceAlongSpline _spline_3 (+ _returnvalue_11 (* (+ _array_index 2) (Variables|Default|GetCartSpacing))) "Local"))) (.Yaw (Math|Rotator|BreakRotator (Spline|GetRotationatDistanceAlongSpline _spline_3 (+ _returnvalue_11 (* (+ _array_index 2) (Variables|Default|GetCartSpacing))) "Local")))) false false))
  ;[1 1 1] Move Front
  (Transformation|SetRelativeLocationAndRotation (Variables|Default|GetFront) (Math|Vector|MakeVector _x _y (+ _z (Variables|Default|GetTrainDeviation))) (Math|Rotator|MakeRotator _roll_2 _pitch_2 _yaw_2) false false)
  ;[1 1 1] Move Back
  (Transformation|SetRelativeLocationAndRotation (Variables|Default|GetBack) (Math|Vector|MakeVector _x_2 _y_2 (+ _z_2 (Variables|Default|GetTrainDeviation))) (Math|Rotator|MakeRotator _roll (* _pitch -1.0) (+ _yaw 1.8e+02)) false false))

(fn CreateTrain
  ;[1 1 1] Choose Cart Mesh
  (for _index (range 0 (- (Variables|Default|GetNumberOfCarts) 1))
    (if (>= (Variables|Default|GetCartNumber) (- (Utilities|Array|Length (Variables|Default|GetCartMeshes)) 1))
      (Variables|Default|SetCartNumber 0)
      (else
        (Variables|Default|SetCartNumber (+ 1 (Variables|Default|GetCartNumber)))))
    ;[1 1 1] Add Trains
    (bind _returnvalue (AddComponent|AddStaticMeshComponent false))
    (Utilities|Array|Add (Variables|Default|GetTrainCarts) _returnvalue)
    (Components|StaticMesh|SetStaticMesh _returnvalue (Utilities|Array|Get(acopy) (Variables|Default|GetCartMeshes) (Variables|Default|GetCartNumber)))))