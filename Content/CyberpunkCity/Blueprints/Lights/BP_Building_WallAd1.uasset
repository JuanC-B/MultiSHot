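; BP_Building_WallAd1 is a wall advertisement prop whose screen shows a selectable or random holo texture.
; The construction script calls Init, which creates a dynamic material instance from ScreenMaterial on the WallAd component.
; It sets the HoloT parameter to the HoloTextures entry at TextureVariation, re-rolled when Random is set, or to Black when DeviceOn is false.
; The event graph holds only unused stubs, with no runtime logic.
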(event EventBeginPlay)

(event Collision|EventActorBeginOverlap
  (params (OtherActor :type Actor%20Object%20Reference)))

(event EventTick
  (params (DeltaSeconds :type Float%20%28single-precision%29)))

(fn ConstructionScript
  (CallFunction|Init))

(fn Init
  (if (Variables|Default|GetRandom)
    (Variables|Default|SetTextureVariation (Math|Random|RandomInteger (Utilities|Array|Length (Variables|Default|GetHoloTextures)))))
  (bind _returnvalue (Rendering|Material|CreateDynamicMaterialInstance (Variables|Default|GetWallAd) 0 (Variables|Default|GetScreenMaterial) "None" :!class /Script/Engine.PrimitiveComponent))
  (Variables|Default|SetVendingMachineMatInst _returnvalue)
  (if (Variables|Default|GetDeviceOn)
    (Rendering|Material|SetTextureParameterValue (Variables|Default|GetVendingMachineMatInst) "HoloT" (Utilities|Array|Get(acopy) (Variables|Default|GetHoloTextures) (Math|Integer|Clamp(Integer) (Variables|Default|GetTextureVariation) 0 (Utilities|Array|Length (Variables|Default|GetHoloTextures)))))
    (else
      (Rendering|Material|SetTextureParameterValue (Variables|Default|GetVendingMachineMatInst) "HoloT" "/Engine/EngineResources/Black.Black"))))