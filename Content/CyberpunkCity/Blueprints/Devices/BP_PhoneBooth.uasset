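; Phone booth prop for the cyberpunk city that varies its color per instance, with no active gameplay logic.
; The construction script runs Init, which uses ColorVariation to index a color array, or rolls that index randomly when Random is set.
; Init creates dynamic materials for the booth and screen meshes, tinting the plastic with the chosen color and the screen with the same color at double intensity.
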(event EventBeginPlay)

(event Collision|EventActorBeginOverlap
  (params (OtherActor :type Actor%20Object%20Reference)))

(event EventTick
  (params (DeltaSeconds :type Float%20%28single-precision%29)))

(fn ConstructionScript
  (CallFunction|Init))

(fn Init
  (bind _sm_phonebooth1 (Variables|Default|GetSM_PhoneBooth1))
  (bind _sm_phonebooth1_sreen (Variables|Default|GetSM_PhoneBooth1_Sreen))
  (if (Variables|Default|GetRandom)
    (Variables|Default|SetColorVariation (Math|Random|RandomInteger (Utilities|Array|Length (Variables|Default|GetPhoneBoothColor)))))
  (bind _returnvalue (Rendering|Material|CreateDynamicMaterialInstance _sm_phonebooth1 0 (Rendering|Material|GetMaterial _sm_phonebooth1 0) "None" :!class /Script/Engine.PrimitiveComponent))
  (Variables|Default|SetPhoneBoothMatInst _returnvalue)
  (bind _returnvalue_2 (Rendering|Material|CreateDynamicMaterialInstance _sm_phonebooth1_sreen 0 (Rendering|Material|GetMaterial _sm_phonebooth1_sreen 0) "None" :!class /Script/Engine.PrimitiveComponent))
  (Variables|Default|SetScreenMatInst _returnvalue_2)
  (Rendering|Material|SetVectorParameterValue (Variables|Default|GetPhoneBoothMatInst) "PlasticColor" (Utilities|Array|Get(acopy) (Variables|Default|GetPhoneBoothColor) (Variables|Default|GetColorVariation)) :!class /Script/Engine.MaterialInstanceDynamic)
  (Rendering|Material|SetVectorParameterValue (Variables|Default|GetScreenMatInst) "MaskedColor" (* (Utilities|Array|Get(acopy) (Variables|Default|GetPhoneBoothColor) (Variables|Default|GetColorVariation)) 2.0) :!class /Script/Engine.MaterialInstanceDynamic))