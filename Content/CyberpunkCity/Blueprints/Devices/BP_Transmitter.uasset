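; BP_Transmitter is a decorative transmitter prop for the Cyberpunk City devices set, with selectable color variations.
; Its construction script runs Init, which optionally picks a random color index when Random is set.
; Init creates a dynamic material instance on the SMTransmitter mesh and sets PlasticColor and PatternColor from two color arrays at that shared index.
; The event graph holds no active logic.
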(event EventBeginPlay)

(event Collision|EventActorBeginOverlap
  (params (OtherActor :type Actor%20Object%20Reference)))

(event EventTick
  (params (DeltaSeconds :type Float%20%28single-precision%29)))

(fn ConstructionScript
  (CallFunction|Init))

(fn Init
  (bind _sm_transmitter (Variables|Default|GetSM_Transmitter))
  (if (Variables|Default|GetRandom)
    (Variables|Default|SetColorVariation (Math|Random|RandomInteger (Utilities|Array|Length (Variables|Default|GetTransmitterColorsA)))))
  (bind _returnvalue (Rendering|Material|CreateDynamicMaterialInstance _sm_transmitter 0 (Rendering|Material|GetMaterial _sm_transmitter 0) "None" :!class /Script/Engine.PrimitiveComponent))
  (Variables|Default|SetTransmitterMatInst _returnvalue)
  (Rendering|Material|SetVectorParameterValue (Variables|Default|GetTransmitterMatInst) "PlasticColor" (Utilities|Array|Get(acopy) (Variables|Default|GetTransmitterColorsA) (Variables|Default|GetColorVariation)) :!class /Script/Engine.MaterialInstanceDynamic)
  (Rendering|Material|SetVectorParameterValue (Variables|Default|GetTransmitterMatInst) "PatternColor" (Utilities|Array|Get(acopy) (Variables|Default|GetTransmitterColorsB) (Variables|Default|GetColorVariation)) :!class /Script/Engine.MaterialInstanceDynamic))