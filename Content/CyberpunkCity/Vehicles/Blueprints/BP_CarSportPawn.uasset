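; BP_CarSportPawn is the sport car vehicle pawn, extending a parent vehicle Blueprint to drive the car's skeletal mesh animation.
; On BeginPlay it caches the mesh's SK_Car_Sport_AnimBP instance.
; Each Tick it passes the steering angle to that AnimBP for the steering wheel.
; Door updates run the parent logic, then send both front door states to the AnimBP through a message call.
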(event EventBeginPlay
  (|CallParentFunction)
  (bind _assk_car_sport_anim_bp (Utilities|Casting|CastToSK_Car_Sport_AnimBP (Components|SkeletalMesh|GetAnimInstance (Variables|Character|GetMesh))))
  (Variables|Default|SetAnimBPRef _assk_car_sport_anim_bp))

(event Collision|EventActorBeginOverlap
  (params (OtherActor :type Actor%20Object%20Reference)))

(event EventTick
  (params (DeltaSeconds :type Float%20%28single-precision%29))
  (|CallParentFunction DeltaSeconds)
  ;[1 1 1] Update Steering Wheel Rotation
  (if (Utilities|IsValid (Variables|Default|GetAnimBPRef))
    (Default|UpdateStreering (Variables|Default|GetAnimBPRef) (Variables|Default|GetSteeringAngle))))

(event EventUpdateVehicleDoors
  ;[1 1 1] Update Doors
  (|CallParentFunction)
  (Class|BPIVehicleAnimInterface|UpdateDoors(Message) (Variables|Default|GetAnimBPRef) (Variables|Default|GetFrontRightDoor) (Variables|Default|GetFrontLeftDoor)))

(fn ConstructionScript
  (|CallParentFunction))