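; Truck variant of a parent vehicle pawn that adds an optional, color-tinted cargo mesh and drives the truck's animation.
; It caches the SK_Car_Truck_AnimBP instance on BeginPlay, feeds it the steering angle each tick and passes front door states on door updates.
; The construction script assigns the cargo mesh and creates a dynamic material instance to set its AlbedoColor from CargoColor.
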(event EventBeginPlay
  (|CallParentFunction)
  (bind _assk_car_truck_anim_bp (Utilities|Casting|CastToSK_Car_Truck_AnimBP (Components|SkeletalMesh|GetAnimInstance (Variables|Character|GetMesh))))
  (Variables|Default|SetAnimationBP _assk_car_truck_anim_bp))

(event Collision|EventActorBeginOverlap
  (params (OtherActor :type Actor%20Object%20Reference)))

(event EventTick
  (params (DeltaSeconds :type Float%20%28single-precision%29))
  (bind _animationbp (Variables|Default|GetAnimationBP))
  (|CallParentFunction DeltaSeconds)
  ;[1 1 1] Update Steering Wheel Rotation
  (if (Utilities|IsValid _animationbp)
    (Default|UpdateStreering _animationbp (Variables|Default|GetSteeringAngle))))

(event EventUpdateVehicleDoors
  ;[1 1 1] Update Doors
  (|CallParentFunction)
  (Class|BPIVehicleAnimInterface|UpdateDoors(Message) (Variables|Default|GetAnimationBP) (Variables|Default|GetFrontRightDoor) (Variables|Default|GetFrontLeftDoor)))

(fn ConstructionScript
  (bind _cargo (Variables|Default|GetCargo))
  (|CallParentFunction)
  ;[1 1 1] Cargo
  (Utilities|IsValid (Variables|Visuals|GetCargoMesh)
    (:Is%20Valid
      (Components|StaticMesh|SetStaticMesh _cargo (Variables|Visuals|GetCargoMesh))
      (bind _returnvalue (Rendering|Material|CreateDynamicMaterialInstance _cargo 0 (Rendering|Material|GetMaterial _cargo 0) "None" :!class /Script/Engine.PrimitiveComponent))
      (bind _output_get (Variables|Visuals|SetCargoMatInst _returnvalue))
      (Rendering|Material|SetVectorParameterValue _output_get "AlbedoColor" (Variables|Visuals|GetCargoColor) :!class /Script/Engine.MaterialInstanceDynamic))))