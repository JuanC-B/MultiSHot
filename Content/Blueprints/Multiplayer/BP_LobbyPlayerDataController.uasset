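; Lobby data controller that hands out unique color IDs to up to three players in random order.
; On BeginPlay, a Server event builds a permutation of 0–2 from a random start and direction using modulo, then passes it through Cast and Local events to fill IdArray and set a ready flag.
; GiveMeColorId returns the next ID, or -1 before assignment.
; AssignateColorOrder duplicates the shuffle locally without setting the flag.
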(event Custom|Server_AssignDefValues
  (Utilities|FlowControl|Sequence
    (:then_0
      (Variables|Default|SetFirstIndexGen (Math|Random|RandomIntegerinRange 0 2))
      (if (Math|Random|RandomBool)
        (Variables|Default|SetSecondIndexGen (Math|Integer|%(Integer) (+ (Variables|Default|GetFirstIndexGen) 1) 3))
        (Variables|Default|SetThirdSecondIndexGen (Math|Integer|%(Integer) (+ (Variables|Default|GetFirstIndexGen) 2) 3))
        (else
          (Variables|Default|SetSecondIndexGen (Math|Integer|%(Integer) (+ (Variables|Default|GetFirstIndexGen) 2) 3))
          (Variables|Default|SetThirdSecondIndexGen (Math|Integer|%(Integer) (+ (Variables|Default|GetFirstIndexGen) 1) 3)))))
    (:then_1
      (CallFunction|CastAssignDefValues (Variables|Default|GetFirstIndexGen) (Variables|Default|GetSecondIndexGen) (Variables|Default|GetThirdSecondIndexGen)))))

(event Custom|Cast_AssignDefValues
  (params (Item :type Integer%20%28by%20ref%29) (Item2 :type Integer%20%28by%20ref%29) (Item3 :type Integer%20%28by%20ref%29))
  (CallFunction|LocalAssignDefValues Item Item2 Item3))

(event Custom|Local_AssignDefValues
  (params (Item :type Integer%20%28by%20ref%29) (Item2 :type Integer%20%28by%20ref%29) (Item3 :type Integer%20%28by%20ref%29))
  (bind _idarray (Variables|Default|GetIdArray))
  (Utilities|Array|SetArrayElem _idarray 0 Item true)
  (Utilities|Array|SetArrayElem _idarray 1 Item2 true)
  (Utilities|Array|SetArrayElem _idarray 2 Item3 true)
  (Variables|Default|SetValuesAssignedFlag true))

(event EventBeginPlay
  (CallFunction|ServerAssignDefValues))

(fn ConstructionScript)

(fn AssignateColorOrder
  (bind _idarray (Variables|Default|GetIdArray))
  (Utilities|FlowControl|Sequence
    (:then_0
      (LocalVariables|SetFirstIndexGen (Math|Random|RandomIntegerinRange 0 2))
      (if (Math|Random|RandomBool)
        (LocalVariables|SetSecondIndexGen (Math|Integer|%(Integer) (+ (LocalVariables|GetFirstIndexGen) 1) 3))
        (LocalVariables|SetThirdSecondIndexGen (Math|Integer|%(Integer) (+ (LocalVariables|GetFirstIndexGen) 2) 3))
        (else
          (LocalVariables|SetSecondIndexGen (Math|Integer|%(Integer) (+ (LocalVariables|GetFirstIndexGen) 2) 3))
          (LocalVariables|SetThirdSecondIndexGen (Math|Integer|%(Integer) (+ (LocalVariables|GetFirstIndexGen) 1) 3)))))
    (:then_1
      (Utilities|Array|SetArrayElem _idarray 0 (LocalVariables|GetFirstIndexGen) true)
      (Utilities|Array|SetArrayElem _idarray 1 (LocalVariables|GetSecondIndexGen) true)
      (Utilities|Array|SetArrayElem _idarray 2 (LocalVariables|GetThirdSecondIndexGen) true))))

(fn GiveMeColorId
  (if (Variables|Default|GetValuesAssignedFlag)
    (LocalVariables|SetidToReturn (Utilities|Array|Get(acopy) (Variables|Default|GetIdArray) (Variables|Default|GetColorsAssignedCount)))
    (Math|Integer|IncrementInt (Variables|Default|GetColorsAssignedCount)
      (:%20%20
        (return (LocalVariables|GetidToReturn))))
    (else
      (return -1))))