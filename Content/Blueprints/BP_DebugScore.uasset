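; BP_DebugScore is a debug actor that shows the total score as "POINTS:" text on a TextRender component.
; It finds and caches the BP_ScoreManager actor on BeginPlay.
; UpdateScoreServer calls UpdateScoreCast, which calls UpdateScoreLocal to rewrite the text from the manager's TotalScore, a chain named for server-to-multicast relay.
; Nothing inside the Blueprint triggers the update.
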(event Custom|Update%20Score%20Local
  (Rendering|Components|TextRender|SetText (Variables|Default|GetTextRender) (Utilities|Text|ToText(String) (Utilities|String|Append "POINTS:" (Utilities|String|ToString(Float) (Variables|/Game/Blueprints/HordeMode/BP_ScoreManager.BP_ScoreManager_C|GetTotalScore (Variables|Default|GetScoreBP)))))))

(event Custom|Update%20Score%20Server
  (CallFunction|UpdateScoreCast))

(event Custom|Update%20Score%20Cast
  (CallFunction|UpdateScoreLocal))

(event EventBeginPlay
  (bind _returnvalue (Actor|GetActorOfClass "/Game/Blueprints/HordeMode/BP_ScoreManager.BP_ScoreManager_C"))
  (Variables|Default|SetScoreBP _returnvalue))

(fn ConstructionScript)