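; Replicated hand socket that shows a colored robotic hand mesh when used, mirrored for left-hand use.
; BeginPlay applies the ColorID color and hides the mesh; Use makes it visible and scales HandSocket by InvertAxis for left hands.
; Visibility and scale pass through Server, Cast and Local events, while the server color event calls the local one directly.
; Color swaps the Albedo texture on a dynamic material instance.
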(event Custom|Use
  (params (isLeft :type Boolean))
  (CallFunction|ServerHide true)
  (CallFunction|ServerSetScale isLeft))

(event Custom|LocalHide
  (params (bNewVisibility :type Boolean))
  ;[1 1 1] Show/Hide (with replication)
  (Rendering|SetVisibility (Variables|Default|GetHand_mesh) bNewVisibility true))

(event Custom|server_setHandColor
  (params (Index :type Integer))
  ;[1 1 1] set hand color
  (CallFunction|LocalSetHandColor Index))

(event Custom|Local_setHandColor
  (params (Index :type Integer))
  ;[1 1 1] set hand color
  (CallFunction|AssignHandColor Index))

(event Custom|Cast_setHandColor
  (params (Index :type Integer))
  ;[1 1 1] set hand color
  (CallFunction|LocalSetHandColor Index))

(event Custom|ServerHide
  (params (bNewVisibility :type Boolean))
  ;[1 1 1] Show/Hide (with replication)
  (CallFunction|CastHide bNewVisibility))

(event Custom|CastHide
  (params (bNewVisibility :type Boolean))
  ;[1 1 1] Show/Hide (with replication)
  (CallFunction|LocalHide bNewVisibility))

(event Custom|Server_SetScale
  (params (isLeft :type Boolean))
  ;[1 1 1] Invert Left
  (CallFunction|CastSetScale isLeft))

(event Custom|Local_SetScale
  (params (isLeft :type Boolean))
  ;[1 1 1] Invert Left
  (Transformation|SetRelativeScale3D (Variables|Default|GetHand_socket) (Math|Vector|SelectVector (Variables|Default|GetInvertAxis) "1.000000,1.000000,1.000000" isLeft)))

(event Custom|Cast_SetScale
  (params (isLeft :type Boolean))
  ;[1 1 1] Invert Left
  (CallFunction|LocalSetScale isLeft))

(event EventBeginPlay
  (CallFunction|ServerSetHandColor (Variables|Default|GetColorID))
  (CallFunction|ServerHide false))

(fn ConstructionScript)

(fn AssignHandColor
  (params (Index :type Integer))
  (bind _hand_mesh (Variables|Default|GetHand_mesh))
  (bind _returnvalue (Rendering|Material|CreateDynamicMaterialInstance _hand_mesh 0 0 "None" :!class /Script/Engine.PrimitiveComponent))
  (LocalVariables|SetMaterialInstance _returnvalue)
  (Rendering|Material|SetTextureParameterValue (LocalVariables|GetMaterialInstance) "Albedo" (Utilities|Select :Index Index :Option%200 "/Game/VRHandsPack/Textures/T_Robotic_BC.T_Robotic_BC" :Option%201 "/Game/VRHandsPack/Textures/T_Robotic_BC_Green.T_Robotic_BC_Green" :Option%202 "/Game/VRHandsPack/Textures/T_Robotic_BC_Blue.T_Robotic_BC_Blue"))
  (Rendering|Material|SetMaterial _hand_mesh 0 (LocalVariables|GetMaterialInstance)))