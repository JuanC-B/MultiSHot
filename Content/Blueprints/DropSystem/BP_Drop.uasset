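; Supply drop actor that falls to a fixed height on a timeline, then explodes with VFX and sound, spawns a random pickup and destroys itself.
; RandomItem rolls ammo, medicine or one of four weapons, with weapon rarity odds set from DiffLevel in the construction script.
; Weapons receive their rarity and matching particles on spawn.
; Fall, spawn and destroy events are split into Server and Local variants.
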(event Custom|Destroy%20Local
  ;[1 1 1] Destroy Early
  (Actor|DestroyActor))

(event Custom|Spawn%20Drop
  ;[0.5585 0.2764 1] Spawn Drop Server/Local
  (CallFunction|SpawnDropServer))

(event Custom|Falldown%20Local
  (bind _startposition (Variables|Default|GetStartPosition))
  ;[0.9144 1 0.04911] Fall Local/Server
  (Components|Timeline|SetPlayRate (Variables|Default|GetFall) 0.2)
  (bind _fall_alpha (Timeline|Fall Play)
    (:Update
      (Transformation|SetWorldLocation (Variables|Debug|GetStaticMeshComponent) (Math|Vector|Lerp(Vector) (Variables|Default|GetStartPosition) (Math|Vector|MakeVector (.x _startposition) (.y _startposition) 5716.061523) _fall_alpha) false false))
    (:Finished
      (CallFunction|SpawnDrop)
      (Actor|DestroyActor))))

(event Custom|Spawn%20Drop%20Server
  (bind _staticmeshcomponent (Variables|Debug|GetStaticMeshComponent))
  (bind _returnvalue (Transformation|GetWorldLocation _staticmeshcomponent))
  (bind (_x _y _z) (Math|Vector|BreakVector _returnvalue))
  (bind _returnvalue_2 (+ _z 1e+02))
  (bind _returnvalue_3 (Math|Conversions|ToTransform(Vector) (Math|Vector|MakeVector _x _y _returnvalue_2)))
  ;[0.5585 0.2764 1] Spawn Drop Server/Local
  (Effects|SpawnEmitteratLocation (Variables|Default|GetExplosion%20Drop%20VFX) _returnvalue)
  (Audio|PlaySoundatLocation (Variables|Default|GetExplosion%20Drop%20SFX) _returnvalue "0, 0, 0" 1.0 1.0 0.0 0 0 0 0)
  (bind (_class _weaponrarity) (CallFunction|RandomItem))
  (Variables|Default|SetSpawnLoc _returnvalue_3)
  (Variables|Default|SetWeapon%20Rarity _weaponrarity)
  (bind _asbp_weapon_master (Utilities|Casting|CastToBP_WeaponMasterClass _class)
    (:then
      (Variables|Default|SetClass _asbp_weapon_master)
      (Variables|Default|SetisWeapon true)
      (bind _returnvalue_4 (Game|SpawnActorfromClass _asbp_weapon_master _returnvalue_3 "Undefined" "MultiplyWithRoot" 0 _weaponrarity "/Game/VRHandsPack/Animations/MannequinHand_Right_Gun.MannequinHand_Right_Gun" 0))
      (Default|SetParticles _returnvalue_4 _weaponrarity))
    (:CastFailed
      (Variables|Default|SetClass _class)
      (Variables|Default|SetisWeapon false)
      (Game|SpawnActorfromClass _class _returnvalue_3 "Undefined" "MultiplyWithRoot" 0 0))))

(event Custom|Falldown
  ;[0.9144 1 0.04911] Fall Local/Server
  (CallFunction|FalldownServer)
  (CallFunction|FalldownLocal))

(event Custom|Destroy
  ;[1 1 1] Destroy Early
  (CallFunction|DestroyServer)
  (CallFunction|DestroyLocal))

(event Custom|Falldown%20Server
  ;[0.9144 1 0.04911] Fall Local/Server
  (CallFunction|FalldownLocal))

(event Custom|Destroy%20Server
  ;[1 1 1] Destroy Early
  (CallFunction|DestroyLocal))

(event EventBeginPlay
  (bind _staticmeshcomponent (Variables|Debug|GetStaticMeshComponent))
  (bind _returnvalue (Transformation|GetWorldLocation _staticmeshcomponent))
  (Variables|Default|SetStartPosition _returnvalue)
  (Audio|PlaySoundatLocation (Variables|Default|GetStart%20Drop%20SFX) _returnvalue "0, 0, 0" 1.0 1.0 0.0 0 0 0 0)
  (CallFunction|Falldown))

(fn ConstructionScript
  (bind _difflevel (Variables|Default|GetDiffLevel))
  (Variables|Default|SetNormalRProb (Utilities|Select :Index _difflevel :Option%200 80 :Option%201 60 :Option%202 55 :Option%203 35 :Option%204 0))
  (Variables|Default|SetRareRProb (Utilities|Select :Index _difflevel :Option%200 20 :Option%201 30 :Option%202 25 :Option%203 35 :Option%204 45))
  (Variables|Default|SetEpicRProb (Utilities|Select :Index _difflevel :Option%200 0 :Option%201 10 :Option%202 15 :Option%203 20 :Option%204 35)))

(fn RandomItem
  (bind _amoprobabilitty (Variables|Default|GetAmoProbabilitty))
  (bind _gunprobability (Variables|Default|GetGunProbability))
  (bind _fusilprobability (Variables|Default|GetFusilProbability))
  (bind _normalrprob (Variables|Default|GetNormalRProb))
  (bind _rarerprob (Variables|Default|GetRareRProb))
  (bind _returnvalue (+ _normalrprob _rarerprob))
  (bind _returnvalue_2 (+ _gunprobability _fusilprobability))
  (bind _output_get (LocalVariables|SetRandomTemporal (Math|Random|RandomIntegerinRange 0 100)))
  (if (< _output_get _amoprobabilitty)
    ;[1 1 1] municion
    (bind _output_get_2 (LocalVariables|SetClassSpawn "/Game/Blueprints/Consumibles/BP_CON_Munition.BP_CON_Munition_C"))
    (return _output_get_2 "NewEnumerator0")
    (elif (< _output_get (+ _amoprobabilitty (Variables|Default|GetHealthProbabilitty)))
      ;[1 1 1] Botiquin
      (bind _output_get_3 (LocalVariables|SetClassSpawn "/Game/Blueprints/Consumibles/BP_CON_Medicine.BP_CON_Medicine_C"))
      (return _output_get_3 "NewEnumerator0")
      (else
        (Utilities|FlowControl|Sequence
          (:then_0
            ;[1 1 1] Rarity Weapon
            (bind _output_get_4 (LocalVariables|SetRandomTemporal (Math|Random|RandomIntegerinRange 0 100)))
            (if (<= _output_get_4 _normalrprob)
              (LocalVariables|SetRarity "NewEnumerator0")
              (elif (<= _output_get_4 _returnvalue)
                (LocalVariables|SetRarity "NewEnumerator1")
                (elif (<= _output_get_4 (+ _returnvalue (Variables|Default|GetEpicRProb)))
                  (LocalVariables|SetRarity "NewEnumerator2")
                  (else
                    (LocalVariables|SetRarity "NewEnumerator3"))))))
          (:then_1
            ;[1 1 1] arma
            (bind _output_get_5 (LocalVariables|SetRandomTemporal (Math|Random|RandomIntegerinRange 0 100)))
            (if (<= _output_get_5 _gunprobability)
              (bind _output_get_6 (LocalVariables|SetClassSpawn "/Game/Blueprints/Weapons/Normal_Weapon/BP_N_Gun.BP_N_Gun_C"))
              (return _output_get_6 (LocalVariables|GetRarity))
              (else
                (bind _output_get_7 (LocalVariables|SetProbabilityValue _returnvalue_2))
                (if (<= _output_get_5 _returnvalue_2)
                  (bind _output_get_8 (LocalVariables|SetClassSpawn "/Game/Blueprints/Weapons/Normal_Weapon/BP_N_Fusil.BP_N_Fusil_C"))
                  (return _output_get_8 (LocalVariables|GetRarity))
                  (else
                    (LocalVariables|SetProbabilityValue (+ _output_get_7 (Variables|Default|GetBazookaProbability)))
                    (if (<= _output_get_5 (+ _output_get_7 (Variables|Default|GetBazookaProbability)))
                      (bind _output_get_9 (LocalVariables|SetClassSpawn "/Game/Blueprints/Weapons/Rocket_Weapon/BP_WM_RocketWeapon.BP_WM_RocketWeapon_C"))
                      (return _output_get_9 (LocalVariables|GetRarity))
                      (else
                        (bind _output_get_10 (LocalVariables|SetClassSpawn "/Game/Blueprints/Weapons/Normal_Weapon/BP_N_Gatling.BP_N_Gatling_C"))
                        (return _output_get_10 (LocalVariables|GetRarity))))))))))))))