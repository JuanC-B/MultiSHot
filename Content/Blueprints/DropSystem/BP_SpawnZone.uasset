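; BP_SpawnZone is a drop spawner that places BP_Drop actors at random positions inside a rectangular area.
; BeginPlay caches four marker component locations as the X and Y bounds and starts a looping one-second timer on SpawnDrop.
; Each spawn uses the root's height and passes DiffLevel to the drop.
; DropManager holds a DropRating counter check, but nothing in this graph calls it.
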(event Custom|DropManager
  (bind _output_get (Variables|Default|SetTimeDrop (+ (Variables|Default|GetTimeDrop) 1.0)))
  (if (== _output_get (Variables|Default|GetDropRating))
    (CallFunction|SpawnDrop)))

(event Custom|SpawnDrop
  (Game|SpawnActorfromClass "/Game/Blueprints/DropSystem/BP_Drop.BP_Drop_C" (Math|Transform|MakeTransform (Math|Vector|MakeVector (Math|Random|RandomFloatinRange (.x (Variables|Default|GetN_Location)) (.x (Variables|Default|GetS_Location))) (Math|Random|RandomFloatinRange (.y (Variables|Default|GetE_Location)) (.y (Variables|Default|GetO_Location))) (.z (Transformation|GetWorldLocation (Variables|Default|GetDefaultSceneRoot)))) "0, 0, 0" "1.000000,1.000000,1.000000") "Undefined" "MultiplyWithRoot" 0 (Variables|Default|GetDiff%20Level) 0))

(event EventBeginPlay
  (Variables|Default|SetN_Location (Transformation|GetWorldLocation (Variables|Default|GetN_Point)))
  (Variables|Default|SetS_Location (Transformation|GetWorldLocation (Variables|Default|GetS_Point)))
  (Variables|Default|SetE_Location (Transformation|GetWorldLocation (Variables|Default|GetE_Point)))
  (Variables|Default|SetO_Location (Transformation|GetWorldLocation (Variables|Default|GetO_Point)))
  (Utilities|Time|SetTimerbyEvent (delegate Custom|SpawnDrop) 1.0 true))

(fn ConstructionScript)