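; BP_Nexo is the Horde Mode Nexus, a damageable structure whose energy shield shows its remaining health.
; SilentDamage lowers Health, then passes it through a server/cast/local event chain with a debug print, or calls death, whose handler is empty here.
; One-shot percentage thresholds recolor the Niagara shield, shorten its lifetime and spawn lightning at low health.
; TryDamage is a stub that deals no damage.
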(event Custom|Server_UpdateLife
  (params (Health :type Float%20%28double-precision%29))
  ;[0.1121 1 0.1281] Health Update
  (CallFunction|CastUpdateLife Health))

(event Custom|Cast_UpdateLife
  (params (Health :type Float%20%28double-precision%29))
  ;[0.1121 1 0.1281] Health Update
  (CallFunction|LocalUpdateLife Health))

(event Custom|Local_UpdateLife
  (params (Health :type Float%20%28double-precision%29))
  ;[0.1121 1 0.1281] Health Update
  (bind _output_get (Variables|Default|SetHealth Health))
  (Development|PrintString (Utilities|String|Append "VIDA NEXO: " (Utilities|String|ToString(Float) _output_get)) true true "(R=0.199755,G=1.000000,B=0.000000,A=1.000000)"))

(event Custom|Server_Die)

(event Custom|AppealNexoLocal
  (bind _n_energyshield (Variables|Default|GetN_EnergyShield))
  (bind _n_energyshield_2 (Variables|Default|GetN_EnergyShield))
  (bind _n_energyshield_3 (Variables|Default|GetN_EnergyShield))
  (bind ___hp (CallFunction|LifeState (Variables|Default|GetHealth)))
  (if (and (<= ___hp 75) (Variables|Default|Get75%25))
    (Variables|Default|Set75%25 false)
    (Class|NiagaraComponent|SetVariableMaterial _n_energyshield_2 "MatInterface" "/Game/MegaMagicVFXBundle/VFX/MagicShieldsVFX/VFX/StylizedVersions/EnergyShieldStylized/Materials/MI_EnergyShieldStylizedYellow.MI_EnergyShieldStylizedYellow")
    (Niagara|SetNiagaraVariable(Float) _n_energyshield_2 "Lifetime" 3.5)
    (elif (and (<= ___hp 50) (Variables|Default|Get50%25))
      (Variables|Default|Set50%25 false)
      (Class|NiagaraComponent|SetVariableMaterial _n_energyshield_3 "MatInterface" "/Game/MegaMagicVFXBundle/VFX/MagicShieldsVFX/VFX/StylizedVersions/EnergyShieldStylized/Materials/MI_EnergyShieldStylizedOrange.MI_EnergyShieldStylizedOrange")
      (Niagara|SetNiagaraVariable(Float) _n_energyshield_3 "Lifetime" 3.0)
      (elif (and (<= ___hp 25) (Variables|Default|Get25%25))
        (Variables|Default|Set25%25 false)
        (Class|NiagaraComponent|SetVariableMaterial _n_energyshield "MatInterface" "/Game/MegaMagicVFXBundle/VFX/MagicShieldsVFX/VFX/StylizedVersions/EnergyShieldStylized/Materials/MI_EnergyShieldStylizedRed.MI_EnergyShieldStylizedRed")
        (Niagara|SetNiagaraVariable(Float) _n_energyshield "Lifetime" 2.5)
        (Niagara|SpawnSystematLocation "/Game/VFX/NS_Lighting_Low.NS_Lighting_Low" (Transformation|GetWorldLocation (Variables|Default|GetThunderPoint1)))
        (elif (and (<= ___hp 10) (Variables|Default|Get10%25))
          (Variables|Default|Set10%25 false)
          (Niagara|SetNiagaraVariable(Float) (Variables|Default|GetN_EnergyShield) "Lifetime" 1.5)
          (Niagara|SpawnSystematLocation "/Game/VFX/NS_Lighting_Low.NS_Lighting_Low" (Transformation|GetWorldLocation (Variables|Default|GetThunderPoint2))))))))

(event Custom|AppealNexo
  (CallFunction|AppealNexoCast))

(event Custom|AppealNexoCast
  (CallFunction|AppealNexoLocal))

(event Custom|TryDamage_1_1
  (params (damage :type Float%20%28double-precision%29) (Location :type Vector) (Player :type BP%20VR%20Character%20Object%20Reference)))

(event EventBeginPlay
  (Variables|Default|SetSphereLoc (Transformation|GetWorldLocation (Variables|Default|GetN_EnergyShield))))

(event Collision|EventActorBeginOverlap
  (params (OtherActor :type Actor%20Object%20Reference)))

(event EventTick
  (params (DeltaSeconds :type Float%20%28single-precision%29)))

(event EventSilentDamage
  (params (damage :type Float%20%28double-precision%29))
  (bind _output_get (Variables|Default|SetHealth (- (Variables|Default|GetHealth) damage)))
  (Utilities|FlowControl|Sequence
    (:then_0
      (if (> _output_get 0.0)
        (CallFunction|ServerUpdateLife (Variables|Default|GetHealth))
        (CallFunction|AppealNexo)
        (if (> (Variables|Default|GetHealth) 0.0)
          _)
        (else
          (CallFunction|ServerDie))))
    (:then_1
      (if (> damage 0.0)
        _))))

(fn ConstructionScript
  (Niagara|SetNiagaraVariable(Float) (Variables|Default|GetN_EnergyShield) "Lifetime" 4.0))

(fn LifeState
  (params (Health :type Float%20%28double-precision%29))
  (return (Math|Float|Truncate (/ 1e+02 (/ (Variables|Default|GetMaxHealth) Health)))))

(fn ImpactPoint
  (return (Transformation|GetWorldLocation (Variables|Default|GetDamageablePoint))))

(fn TryDamage
  (params (damage :type Float%20%28double-precision%29) (Location :type Vector :default "0, 0, 0"))
  (return 0.0 false))