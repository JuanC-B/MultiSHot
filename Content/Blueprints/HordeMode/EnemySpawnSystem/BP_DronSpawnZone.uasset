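; Spawn zone actor for Horde Mode that spawns drone enemies along the edges of a rectangle.
; BeginPlay runs the BeginReplicate event chain, which caches the NPoint and SPoint corners and the actor's center.
; SpawnDrone maps an enemy type to a BP_NormalEnemy subclass and passes it difficulty, mini-boss flag and center point.
; RandomLocationSpawn picks one of the four edges and a random point along it, while height comes from the root.
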(event Custom|BeginReplicateLocal
  (Variables|Default|SetN_Location (Transformation|GetWorldLocation (Variables|Default|GetN_Point)))
  (Variables|Default|SetS_Location (Transformation|GetWorldLocation (Variables|Default|GetS_Point)))
  (Variables|Default|SetCenterLocation (Transformation|GetActorLocation)))

(event Custom|SpawnDrone
  (params (Class :type ENUM_MinionType%20Enum :default "NewEnumerator0") (Dif%20Level :type Integer) (isMiniBoss :type Boolean))
  (bind _location (CallFunction|RandomLocationSpawn))
  (bind _asbp_normal_enemy (Utilities|Casting|CastToBP_NormalEnemyClass (Utilities|Select :Index Class :NewEnumerator0 "/Game/Blueprints/Damageable/Enemy/BP_NE_Rafaga/BP_NE_Rafaga.BP_NE_Rafaga_C" :NewEnumerator1 "/Game/Blueprints/Damageable/Enemy/BP_NE_Explosive/BP_NE_Explosive.BP_NE_Explosive_C" :NewEnumerator2 "/Game/Blueprints/Damageable/Enemy/BP_NE_Sniper/BP_NE_Sniper.BP_NE_Sniper_C" :NewEnumerator3 "/Game/Blueprints/Damageable/Enemy/BP_NE_Bombs/BP_NE_Bombs.BP_NE_Bombs_C" :NewEnumerator4 "/Game/Blueprints/Damageable/Enemy/BP_NE_Enjambre/BP_NE_EnjambreEnemy.BP_NE_EnjambreEnemy_C")))
  (Game|SpawnActorfromClass _asbp_normal_enemy (Math|Transform|MakeTransform (Math|Vector|MakeVector (.x _location) (.y _location) (.z (Transformation|GetWorldLocation (Variables|Default|GetDefaultSceneRoot)))) "0, 0, 0" "1.000000,1.000000,1.000000") "AlwaysSpawn" "MultiplyWithRoot" 0 (Variables|Default|GetCenterLocation) Dif%20Level isMiniBoss 0))

(event Custom|BeginReplicate
  (CallFunction|BeginReplicateServer))

(event Custom|BeginReplicateServer
  (CallFunction|BeginReplicateLocal))

(event EventBeginPlay
  (CallFunction|BeginReplicate))

(fn ConstructionScript)

(fn RandomLocationSpawn
  (bind _returnvalue (Math|Random|RandomIntegerinRange 1 2))
  (bind _n_location (Variables|Default|GetN_Location))
  (bind _s_location (Variables|Default|GetS_Location))
  (bind _returnvalue_2 (== _returnvalue 1))
  (if (== (Math|Random|RandomIntegerinRange 1 2) 1)
    (if _returnvalue_2
      (LocalVariables|SetDestiny (Math|Vector|MakeVector (Math|Random|RandomFloatinRange (.x _n_location) (.x _s_location)) (.y _n_location) 0.0))
      (else
        (LocalVariables|SetDestiny (Math|Vector|MakeVector (.x _n_location) (Math|Random|RandomFloatinRange (.y _s_location) (.y _n_location)) 0.0))))
    (elif _returnvalue_2
      (LocalVariables|SetDestiny (Math|Vector|MakeVector (Math|Random|RandomFloatinRange (.x _s_location) (.x _n_location)) (.y _s_location) 0.0))
      (else
        (LocalVariables|SetDestiny (Math|Vector|MakeVector (.x _s_location) (Math|Random|RandomFloatinRange (.y _s_location) (.y _n_location)) 0.0)))))
  (return (LocalVariables|GetDestiny)))