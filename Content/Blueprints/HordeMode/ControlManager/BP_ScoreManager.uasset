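; BP_ScoreManager tracks team and per-player score and kills in Horde Mode, and triggers drops at score milestones.
; Score updates apply locally and relay through Server and Cast events, which skip the locally controlled player to avoid double counting.
; The server path adds to the total, refreshes BP_DebugScore, and has BP_SpawnZone spawn a drop whenever accumulated points reach DropPoints, carrying over the remainder.
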(event Custom|PlayerScoreUpdateLocal
  (params (Player :type BP%20VR%20Character%20Object%20Reference) (Score :type Float%20%28double-precision%29))
  ;[1 0.3615 0.2012] INCREMENT INDIVIDUAL SCORE
  (Variables|/Game/Blueprints/BP_VRCharacter__.BP_VRCharacter___C|SetScore Player (+ Score (Variables|/Game/Blueprints/BP_VRCharacter__.BP_VRCharacter___C|GetScore Player))))

(event Custom|PlayerScoreUpdate
  (params (Player :type BP%20VR%20Character%20Object%20Reference) (Score :type Float%20%28double-precision%29))
  ;[1 0.3615 0.2012] INCREMENT INDIVIDUAL SCORE
  (CallFunction|PlayerScoreUpdateServer Player Score)
  (CallFunction|PlayerScoreUpdateLocal Player Score)
  (CallFunction|UpdateTotalScore Score))

(event Custom|DeadCount
  (params (Player :type BP%20VR%20Character%20Object%20Reference))
  ;[1 0 0.01929] KILLS COUNT
  (CallFunction|DeadCountServer)
  (CallFunction|DeadCountIndividualServer Player))

(event Custom|DeadCountIndividualServer
  (params (Character :type BP%20VR%20Character%20Object%20Reference))
  ;[1 0 0.01929] KILLS COUNT
  (bind _result (Math|Integer|IncrementInt (Variables|/Game/Blueprints/BP_VRCharacter__.BP_VRCharacter___C|GetKills Character))
    (:%20%20
      (Variables|/Game/Blueprints/BP_VRCharacter__.BP_VRCharacter___C|SetKills Character _result))))

(event Custom|BeginPlayCast
  ;[1 1 1] BeginPlay Replication
  (CallFunction|BeginPlayLocal))

(event Custom|DeadCountServer
  ;[1 0 0.01929] KILLS COUNT
  (bind _result (Math|Integer|IncrementInt (Variables|Default|GetKills))
    (:%20%20
      (Variables|Default|SetKills _result))))

(event Custom|ScoreDropServer
  (params (Score :type Float%20%28double-precision%29))
  ;[0.5014 0.08239 1] ScoreServerTotalUpdate
  (Variables|Default|SetNextDrop (- Score (Variables|Default|GetDropPoints)))
  (Default|SpawnDrop (Variables|Default|GetDropSpawner)))

(event Custom|BeginPlayLocal
  ;[1 1 1] BeginPlay Replication
  (bind _returnvalue (Actor|GetActorOfClass "/Game/Blueprints/DropSystem/BP_SpawnZone.BP_SpawnZone_C"))
  (Variables|Default|SetDropSpawner _returnvalue)
  (bind _returnvalue_2 (Actor|GetActorOfClass "/Game/Blueprints/BP_DebugScore.BP_DebugScore_C"))
  (Variables|Default|SetDebugScore _returnvalue_2))

(event Custom|PlayerScoreUpdateServer
  (params (Player :type BP%20VR%20Character%20Object%20Reference) (Score :type Float%20%28double-precision%29))
  ;[1 0.3615 0.2012] INCREMENT INDIVIDUAL SCORE
  (CallFunction|PlayerScroreUpdateCast Player Score))

(event Custom|UpdateTotalScore
  (params (Score :type Float%20%28double-precision%29))
  ;[0.5014 0.08239 1] ScoreServerTotalUpdate
  (CallFunction|UpdateTotalScoreServer Score))

(event Custom|PlayerScroreUpdateCast
  (params (Player :type BP%20VR%20Character%20Object%20Reference) (Score :type Float%20%28double-precision%29))
  ;[1 0.3615 0.2012] INCREMENT INDIVIDUAL SCORE
  (if (not (Pawn|IsLocallyControlled Player))
    (CallFunction|PlayerScoreUpdateLocal Player Score)))

(event Custom|BeginPlayRep
  ;[1 1 1] BeginPlay Replication
  (CallFunction|BeginPlayServer))

(event Custom|UpdateTotalScoreServer
  (params (Score :type Float%20%28double-precision%29))
  ;[0.5014 0.08239 1] ScoreServerTotalUpdate
  (bind _newscore (CallFunction|CalculateTotalScore Score))
  (Variables|Default|SetTotalScore _newscore)
  (Default|UpdateScoreServer (Variables|Default|GetDebugScore))
  (bind _output_get (Variables|Default|SetNextDrop (+ Score (Variables|Default|GetNextDrop))))
  (if (>= _output_get (Variables|Default|GetDropPoints))
    (CallFunction|ScoreDropServer _output_get)))

(event Custom|BeginPlayServer
  ;[1 1 1] BeginPlay Replication
  (CallFunction|BeginPlayCast))

(event EventBeginPlay
  ;[1 1 1] BeginPlay Replication
  (CallFunction|BeginPlayRep))

(fn ConstructionScript)

(fn CalculateTotalScore
  (params (Score :type Float%20%28double-precision%29))
  (return (+ Score (Variables|Default|GetTotalScore))))