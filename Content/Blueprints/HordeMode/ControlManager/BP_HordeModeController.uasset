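; BP_HordeModeController sets up a VR horde mode session when play begins.
; After a short delay it counts the VR characters and spawns a BP_N_Gun with particles set for each at the weapon spawn points.
; A further delay in the spawn loop leads to calling Trigger on the ToTriggerOnStart actors through I_Triggereable.
; ReturnAmountPlayerData exposes the stored player count.
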(event EventBeginPlay
  (Utilities|FlowControl|Delay 1.0)
  (bind _outactors (Actor|GetAllActorsOfClass "/Game/Blueprints/BP_VRCharacter__.BP_VRCharacter___C"))
  (bind _output_get (Variables|Default|SetAmountOfPlayers (Utilities|Array|Length _outactors)))
  (for _index (range 0 (- _output_get 1))
    (bind _returnvalue (Game|SpawnActorfromClass "/Game/Blueprints/Weapons/Normal_Weapon/BP_N_Gun.BP_N_Gun_C" (Math|Transform|MakeTransform (Transformation|GetWorldLocation (Utilities|Array|Get(acopy) (Utilities|Array|MakeArray (Variables|Default|GetWeaponSpawn1) (Variables|Default|GetWeaponSpawn2) (Variables|Default|GetWeaponSpawn3)) _index)) "0, 0, 0" "1.000000,1.000000,1.000000") "Undefined" "MultiplyWithRoot" 0 "NewEnumerator0" "/Game/VRHandsPack/Animations/MannequinHand_Right_Gun.MannequinHand_Right_Gun" 0))
    (Default|SetParticles _returnvalue "NewEnumerator0")
    (Utilities|FlowControl|Delay 5.0)
    (for _array_element (Variables|Default|GetToTriggerOnStart)
      (bind _asi_triggereable (Utilities|Casting|CastToI_Triggereable _array_element))
      (Default|Trigger _asi_triggereable))))

(fn ConstructionScript)

(fn ReturnAmountPlayerData
  (return (Variables|Default|GetAmountOfPlayers)))