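; BP_HordeModeController is the horde mode controller that handles start-of-match setup.
; One second after BeginPlay, it stores an actor count as AmountOfPlayers.
; It then spawns a gun at each of its three WeaponSpawn components and sets each gun's particles.
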(event EventBeginPlay
  (Utilities|FlowControl|Delay 1.0)
  (bind _outactors (Actor|GetAllActorsOfClass 0))
  (Variables|Default|SetAmountOfPlayers (Utilities|Array|Length _outactors))
  (for _index (range 0 (- 3 1))
    (bind _returnvalue (Game|SpawnActorfromClass "/Game/Blueprints/Weapons/Normal_Weapon/BP_N_Gun.BP_N_Gun_C" (Math|Transform|MakeTransform (Transformation|GetWorldLocation (Utilities|Array|Get(acopy) (Utilities|Array|MakeArray (Variables|Default|GetWeaponSpawn1) (Variables|Default|GetWeaponSpawn2) (Variables|Default|GetWeaponSpawn3)) _index)) "0, 0, 0" "1.000000,1.000000,1.000000") "Undefined" "MultiplyWithRoot" 0 "NewEnumerator0" 0))
    (Default|SetParticles _returnvalue "NewEnumerator0")))

(fn ConstructionScript)