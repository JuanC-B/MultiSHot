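; BP_DeadController tracks a count of dead tokens for Boss Mode, apparently one per dead player.
; On BeginPlay it hands off to server-named events, reading the token total from BP_HordeModeController's player data count through the I_ControlManager interface.
; GiveToken_Server increments the count and ReturnToken_Server decrements it.
; The check for the count reaching the total has no action attached yet.
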(event Custom|BeginPlay_Server
  ;[0 0.09461 1] Begin Replicacion
  (Utilities|FlowControl|Sequence
    (:then_0
      (bind _returnvalue (Actor|GetActorOfClass "/Game/Blueprints/HordeMode/ControlManager/BP_HordeModeController.BP_HordeModeController_C"))
      (bind _asi_control_manager (Utilities|Casting|CastToI_ControlManager _returnvalue))
      (bind _amountplayers (Default|ReturnAmountPlayerData _asi_control_manager))
      (Variables|Default|SetTotalDeadTokens _amountplayers))))

(event Custom|ReturnToken_Server
  ;[1 0.2825 0.5913] Token Logic
  (bind _result (Math|Integer|DecrementInt (Variables|Default|GetDeadTokens))
    (:%20%20
      (Variables|Default|SetDeadTokens _result))))

(event Custom|GiveToken_Server
  ;[1 0.2825 0.5913] Token Logic
  (bind _result (Math|Integer|IncrementInt (Variables|Default|GetDeadTokens))
    (:%20%20
      (bind _output_get (Variables|Default|SetDeadTokens _result))
      (if (== (Variables|Default|GetTotalDeadTokens) _output_get)
        _))))

(event EventBeginPlay
  ;[0 0.09461 1] Begin Replicacion
  (CallFunction|BeginPlayServer))

(fn ConstructionScript)