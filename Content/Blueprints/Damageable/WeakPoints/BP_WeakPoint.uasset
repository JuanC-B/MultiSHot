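; BP_WeakPoint is a destructible weak point actor that loses health when hit and triggers its linked VulnerableObject when destroyed.
; TryDamage subtracts damage, spawns a hit effect at the impact location, and passes the new health through a Server-to-Cast event chain.
; At zero health or below, a similar DeadServer, DeadCast, DeadLocal chain triggers the VulnerableObject and destroys the actor.
; Health is computed by the caller before being relayed, and the hit effect stays outside that chain.
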(event Custom|DeadServer
  ;[0 0 0] WEAKPOINTS DESTROYED
  (CallFunction|DeadCast))

(event Custom|DeadCast
  ;[0 0 0] WEAKPOINTS DESTROYED
  (CallFunction|DeadLocal))

(event Custom|DamageServer
  (params (Vit%20Update :type Float%20%28double-precision%29))
  ;[0 0 0] TryDamage Weak Point
  (CallFunction|DamageCast Vit%20Update))

(event Custom|DamageCast
  (params (Vit%20Update :type Float%20%28double-precision%29))
  ;[0 0 0] TryDamage Weak Point
  (CallFunction|VitUpdate Vit%20Update))

(event Custom|VitUpdate
  (params (VitUpdate :type Float%20%28double-precision%29))
  ;[0 0 0] TryDamage Weak Point
  (Variables|Default|SetHealthPoints VitUpdate))

(event Custom|DeadLocal
  ;[0 0 0] WEAKPOINTS DESTROYED
  (Default|Trigger (Variables|Default|GetVulnerableObject))
  (Actor|DestroyActor))

(event EventBeginPlay)

(event Collision|EventActorBeginOverlap
  (params (OtherActor :type Actor%20Object%20Reference)))

(event EventTick
  (params (DeltaSeconds :type Float%20%28single-precision%29)))

(event EventTryDamage
  (params (damage :type Float%20%28double-precision%29) (Location :type Vector :default "0, 0, 0"))
  ;[0 0 0] TryDamage Weak Point
  (bind _output_get (Variables|Default|SetHealthPoints (- (Variables|Default|GetHealthPoints) damage)))
  (CallFunction|DamageServer _output_get)
  (Effects|SpawnEmitteratLocation (Variables|Default|GetVFX%20Normal%20Damage) Location)
  (if (<= (Variables|Default|GetHealthPoints) 0.0)
    (CallFunction|DeadServer)))

(fn ConstructionScript)