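; Explosion actor that deals area damage shortly after spawning.
; BeginPlay passes through a server-to-replicate-named event chain that shows either the Niagara effect or the sphere, based on ShowParticle.
; After a brief delay it sizes the sphere to Radious and calls SilentDamage on overlapping I_Damageable actors, skipping InstigatorToIgnore.
; The delayed self-destruct runs from inside that loop, so it depends on finding a damageable overlap.
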(event Custom|ReplicateBeginplay
  (CallFunction|LocalBegin))

(event Custom|LocalBegin
  (bind _showparticle (Variables|Default|GetShowParticle))
  (Development|SetHiddeninGame (Variables|Default|GetNiagara) (not _showparticle) false)
  (Development|SetHiddeninGame (Variables|Default|GetSphere) _showparticle false))

(event Custom|BeginServer
  (CallFunction|ReplicateBeginplay))

(event EventBeginPlay
  (bind _sphere (Variables|Default|GetSphere))
  (bind _overlappingactors (Collision|GetOverlappingActors _sphere 0 :!class /Script/Engine.PrimitiveComponent))
  (CallFunction|BeginServer)
  (Utilities|FlowControl|Delay 0.05)
  (Components|Sphere|SetSphereRadius _sphere (Variables|Default|GetRadious) true)
  (if (>= (Utilities|Array|Length _overlappingactors) 0)
    (for _index (range 0 (Utilities|Array|LastIndex _overlappingactors))
      (bind _asi_damageable (Utilities|Casting|CastToI_Damageable (Utilities|Array|Get(acopy) _overlappingactors _index)))
      (if (not (== (Utilities|Array|Get(acopy) _overlappingactors _index) (Variables|Default|GetInstigatorToIgnore)))
        (Default|SilentDamage _asi_damageable (Variables|Default|GetDamage))))
    (Utilities|FlowControl|Delay 1.0)
    (Actor|DestroyActor)))

(fn ConstructionScript
  (bind _showparticle (Variables|Default|GetShowParticle))
  (Components|Activation|SetAutoActivate (Variables|Default|GetNiagara) _showparticle)
  (Development|SetHiddeninGame (Variables|Default|GetSphere) _showparticle false))