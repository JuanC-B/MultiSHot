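; Enemy drone that rises at spawn, keeps turning toward the Nexo and moves around it at a radius.
; A Road timeline lifts it, then timers drive random arc hops through NormalMove and an Attack chain whose local event is empty.
; TryDamage plays effects and lowers Health through Server/Cast/Local event chains.
; Death destroys it with effects and increments the drone spawn zone's counter, triggering a loot drop every fifth kill.
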(event Custom|RotationLocal
  ;[1 1 1] Rotation - Faced Nexo ¿Timeline?
  (Transformation|SetActorRotation (Math|Rotator|FindLookatRotation (Transformation|GetWorldLocation (Variables|Debug|GetStaticMeshComponent)) (Transformation|GetWorldLocation (Variables|/Script/Engine.Actor|GetRootComponent (Variables|Default|GetNexo))))))

(event Custom|HealthUpdateLocal
  (params (Health :type Float%20%28double-precision%29))
  ;[0.2645 1 0.3567] HealthUpdate Server 4FIX
  (Variables|Default|SetHealth Health))

(event Custom|AttackLocal
  ;[1 1 1] Attack Events
)

(event Custom|DeadCast
  ;[0.821 0.1369 1] Dead Server Local / Include Point LOGIC
  (CallFunction|DeadLocal))

(event Custom|Attack
  ;[1 1 1] Attack Events
  (CallFunction|AttackCast))

(event Custom|AttackCast
  ;[1 1 1] Attack Events
  (CallFunction|AttackLocal))

(event Custom|DamageServer
  (params (Damage :type Float%20%28double-precision%29) (Location :type Vector))
  ;[0.0603 0.4365 1] Recibe Damage Method
  (Effects|SpawnEmitteratLocation (Variables|Default|GetVFXDamage) Location)
  (Audio|PlaySoundatLocation (Variables|Default|GetSFXDamage) Location "0, 0, 0" 1.0 1.0 0.0 0 0 0 0)
  (bind _output_get (Variables|Default|SetHealth (- (Variables|Default|GetHealth) Damage)))
  (if (<= _output_get 0.0)
    (CallFunction|DeadServer)
    (else
      (CallFunction|HealthUpdateServer _output_get))))

(event Custom|HealthUpdateServer
  (params (Health :type Float%20%28double-precision%29))
  ;[0.2645 1 0.3567] HealthUpdate Server 4FIX
  (CallFunction|HealthUpdateCast Health))

(event Custom|RotationServer
  ;[1 1 1] Rotation - Faced Nexo ¿Timeline?
  (CallFunction|RotationCast))

(event Custom|HealthUpdateCast
  (params (Health :type Float%20%28double-precision%29))
  ;[0.2645 1 0.3567] HealthUpdate Server 4FIX
  (CallFunction|HealthUpdateLocal Health))

(event Custom|EnemyMovement
  (params (Position :type Vector))
  ;[1 0.1352 0.265] EnemySetup
  (bind _road (Timeline|Road Play)
    (:Update
      (Transformation|SetWorldLocation (Variables|Debug|GetStaticMeshComponent) (Math|Vector|Lerp(Vector) (Variables|Default|GetPosition%20Start) Position _road) false false))
    (:Finished
      (bind _returnvalue (Utilities|Time|SetTimerbyEvent (delegate Custom|Movement) (Variables|Default|GetMoveCooldown) true))
      (Variables|Default|SetMovementEvent _returnvalue)
      (Utilities|Time|SetTimerbyEvent (delegate Custom|Attack) (Variables|Default|GetAttackCooldown) true))))

(event Custom|DeadLocal
  (bind _staticmeshcomponent (Variables|Debug|GetStaticMeshComponent))
  (bind _returnvalue (Transformation|GetWorldLocation _staticmeshcomponent))
  ;[0.821 0.1369 1] Dead Server Local / Include Point LOGIC
  (Effects|SpawnEmitteratLocation (Variables|Default|GetVFX%20Destroy%20Dron) _returnvalue)
  (Audio|PlaySoundatLocation (Variables|Default|GetSFX%20Destroy%20Dron) _returnvalue "0, 0, 0" 1.0 (Math|Random|RandomFloatinRange 0.8 1.2) 0.0 "/Game/VRE/Core/Character/VOIPAtten.VOIPAtten" 0 0 0)
  (Actor|DestroyActor))

(event Custom|RotationCast
  ;[1 1 1] Rotation - Faced Nexo ¿Timeline?
  (CallFunction|RotationLocal))

(event Custom|Movement
  ;[0.06105 1 0.9502] Radious Movement
  (bind _output_get (Variables|Default|SetPositionMove (Transformation|GetWorldLocation (Variables|Debug|GetStaticMeshComponent))))
  (Components|Timeline|SetPlayRate (Variables|Default|GetNormalMove) (Variables|Default|GetPlayRateMovement))
  (bind (_x _y) (CallFunction|CalculateNextPointtoMove _output_get (Variables|Default|GetRadious) (Variables|Default|GetMaximum%20Movement) (Variables|Default|GetMinimum%20Movement)))
  (bind _newtrack_0 (Timeline|NormalMove PlayFromStart)
    (:Update
      (Transformation|SetActorLocation (Math|Vector|Lerp(Vector) (Variables|Default|GetPositionMove) (Math|Vector|MakeVector _x _y 0.0) _newtrack_0) false false))))

(event Custom|DeadServer
  (bind _spawndrons (Variables|Default|GetSpawnDrons))
  ;[0.821 0.1369 1] Dead Server Local / Include Point LOGIC
  (CallFunction|DeadCast)
  (bind _result (Math|Integer|IncrementInt (Variables|/Game/Blueprints/HordeMode/BP_DronSpawnZone.BP_DronSpawnZone_C|GetDronDrops _spawndrons))
    (:%20%20
      (bind _output_get (Variables|/Game/Blueprints/HordeMode/BP_DronSpawnZone.BP_DronSpawnZone_C|SetDronDrops _spawndrons _result))
      (if (== _output_get 5)
        (Variables|/Game/Blueprints/HordeMode/BP_DronSpawnZone.BP_DronSpawnZone_C|SetDronDrops (Variables|Default|GetSpawnDrons) 0)
        (Default|SpawnDrop (Variables|Default|GetSpawnLoot))))))

(event EventBeginPlay
  (bind _staticmeshcomponent (Variables|Debug|GetStaticMeshComponent))
  (bind _returnvalue (Transformation|GetWorldLocation _staticmeshcomponent))
  (bind (_x _y _z) (Math|Vector|BreakVector _returnvalue))
  (Utilities|FlowControl|Sequence
    (:then_0
      (bind _returnvalue_2 (Actor|GetActorOfClass "/Game/Blueprints/HordeMode/BP_Nexo.BP_Nexo_C"))
      (Variables|Default|SetNexo _returnvalue_2)
      (bind _returnvalue_3 (Actor|GetActorOfClass "/Game/Blueprints/DropSystem/BP_SpawnZone.BP_SpawnZone_C"))
      (Variables|Default|SetSpawnLoot _returnvalue_3)
      (bind _returnvalue_4 (Actor|GetActorOfClass "/Game/Blueprints/HordeMode/BP_DronSpawnZone.BP_DronSpawnZone_C"))
      (Variables|Default|SetSpawnDrons _returnvalue_4))
    (:then_1
      (Utilities|Time|SetTimerbyEvent (delegate Custom|RotationServer) 0.2 true)
      (Variables|Default|SetPosition%20Start _returnvalue)
      (bind _outhit (Collision|LineTraceByChannel _returnvalue (Math|Vector|MakeVector _x _y (+ _z 2e+03)) "TraceTypeQuery2" false 0 "ForOneFrame"))
      (CallFunction|EnemyMovement (.traceend _outhit)))))

(event EventTryDamage
  (params (damage :type Float%20%28double-precision%29) (Location :type Vector :default "0, 0, 0") (Player :type BP%20VR%20Character%20Object%20Reference))
  ;[0.0603 0.4365 1] Recibe Damage Method
  (CallFunction|DamageServer damage Location))

(fn ConstructionScript)

(fn CalculateNextPointtoMove
  (params (CurrentLocation :type Vector) (Radious :type Float%20%28double-precision%29) (MaximumMovement :type Float%20%28double-precision%29) (MinimumMovement :type Float%20%28double-precision%29))
  (bind (_x _y) (Math|Vector|BreakVector CurrentLocation))
  (bind _returnvalue (Math|Random|RandomBool))
  (bind _returnvalue_2 (Math|Random|RandomFloatinRange MinimumMovement MaximumMovement))
  (bind _centerpoint (Variables|Default|GetCenterPoint))
  (bind _returnvalue_3 (Math|Vector2D|MakeVector2D _x _y))
  (bind _returnvalue_4 (Math|Float|SelectFloat 1.0 -1.0 _returnvalue))
  (bind (_x_2 _y_2) (Math|Vector|BreakVector _centerpoint))
  (bind _returnvalue_5 (Math|Vector2D|MakeVector2D _x_2 _y_2))
  (bind _returnvalue_6 (* _returnvalue_2 _returnvalue_4))
  (bind _returnvalue_7 (- _returnvalue_3 _returnvalue_5))
  (bind _returnvalue_8 (Math|Vector2D|Normalize2D _returnvalue_7))
  (bind _returnvalue_9 (Math|Vector2D|DotProduct(2D) _returnvalue_8 "(X=0.000000,Y=1.000000)"))
  (bind _returnvalue_10 (Class|KismetMathLibrary|DegAcos _returnvalue_9))
  (bind _returnvalue_11 (+ _returnvalue_10 _returnvalue_6))
  (return (* (Math|Trig|Sin(Degrees) _returnvalue_11) Radious) (* (Math|Trig|Cos(Degrees) _returnvalue_11) Radious)))