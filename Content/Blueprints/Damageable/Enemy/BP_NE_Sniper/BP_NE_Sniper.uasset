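; Sniper enemy that telegraphs its attack with an aiming laser, then damages its target with an explosive shot.
; AttackLocal plays the ShotLogic timeline, timed from MoveCooldown, to spawn the laser, sweep its end around the impact point and animate its width.
; On finish, a trace only places the explosion, while damage always applies to the target.
; The construction script scales cooldowns and damage by difficulty, randomizing attack cooldown.
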(event EventBeginPlay
  (|CallParentFunction) ; This node is disabled and will not be called.\nDrag off pins to build functionality.
)

(event Collision|EventActorBeginOverlap
  (params (OtherActor :type Actor%20Object%20Reference)))

(event EventAttackLocal
  (bind _target (Variables|Default|GetTarget))
  (bind _angledispersion (Variables|Default|GetAngleDispersion))
  (bind _returnvalue (* _angledispersion -1.0))
  (|CallParentFunction)
  (bind _point (Default|ImpactPoint _target))
  (Components|Timeline|SetPlayRate (Variables|Default|GetShotLogic) (/ 1.0 (- (Variables|Default|GetMoveCooldown) 2.0)))
  (bind (_direction _x _y _width) (Timeline|ShotLogic PlayFromStart)
    (:Update
      (Niagara|SetNiagaraVariable(Vector3) (Variables|Default|GetBeam) "Beam End" (Math|Vector|MakeVector (Math|Float|Lerp (+ (.x _point) _angledispersion) (+ (.x _point) _returnvalue) _x) (Math|Float|Lerp (+ (.y _point) _angledispersion) (+ (.y _point) _returnvalue) _y) (.z _point)))
      (Niagara|SetNiagaraVariable(Float) (Variables|Default|GetBeam) "BeamWidth" (Math|Float|Lerp 0.332528 (Variables|Default|GetBeamWidth) _width)))
    (:Finished
      (bind _point_2 (Default|ImpactPoint (Variables|Default|GetTarget)))
      (Components|DestroyComponent (Variables|Default|GetBeam))
      (bind _outhit (Collision|LineTraceByChannel (Transformation|GetWorldLocation (Variables|Default|GetShotPoint)) _point_2 "TraceTypeQuery5" false 0 "ForDuration" true "(R=1.000000,G=0.000000,B=0.000000,A=1.000000)" "(R=0.000000,G=1.000000,B=0.000000,A=1.000000)" 0.2))
      (bind _returnvalue_2 (Niagara|SpawnSystematLocation "/Game/VFX/NS_Explosion_B.NS_Explosion_B" (.location _outhit)))
      (Default|SilentDamage _target (Variables|Default|GetDamage))
      (Utilities|FlowControl|Delay 1.0)
      (Components|DestroyComponent _returnvalue_2))
    (:Spawn%20Laser
      (bind _returnvalue_3 (Niagara|SpawnSystematLocation "/Game/VFX/NS_SniperLaser.NS_SniperLaser" (Transformation|GetWorldLocation (Variables|Default|GetShotPoint))))
      (bind _output_get (Variables|Default|SetBeam _returnvalue_3))
      (Transformation|AttachComponentToComponent _output_get (Variables|Default|GetShotPoint) "ShotPoint" "KeepRelative" "KeepRelative" "KeepRelative" false))))

(fn ConstructionScript
  (Variables|Default|SetMoveCooldown (Utilities|Select :Index (Variables|Default|GetDif%20Level) :Option%200 8.0 :Option%201 7.0 :Option%202 6.5 :Option%203 6.0 :Option%204 7.0))
  (bind _output_get (Variables|Default|SetAttackCooldown (+ (Math|Random|RandomFloatinRange 1.0 2.0) (Utilities|Select :Index (Variables|Default|GetDif%20Level) :Option%200 1e+01 :Option%201 9.0 :Option%202 8.0 :Option%203 7.0 :Option%204 6.0))))
  (Variables|Default|SetTimeMoving (- _output_get 2.0))
  (Variables|Default|SetMaximum%20Movement 1.8e+02)
  (Variables|Default|SetDamage (Utilities|Select :Index (Variables|Default|GetDif%20Level) :Option%200 8.0 :Option%201 16.0 :Option%202 2e+01 :Option%203 24.0 :Option%204 3e+01)))