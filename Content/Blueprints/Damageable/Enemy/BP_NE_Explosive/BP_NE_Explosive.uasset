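; Explosive enemy, derived from a parent enemy class, that closes in on its target and detonates on touching a player-side damageable.
; A looping timer re-aims at the target's impact point, and a duration-scaled timeline lerps the actor one fixed-distance step toward it without sweeping.
; Sphere overlap calls DeadServer, while DeadLocal spawns a damaging BP_Explosion and destroys the actor.
; Difficulty level selects the step distance.
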(event OnComponentBeginOverlap(Sphere)
  (params (OverlappedComponent :type Primitive%20Component%20Object%20Reference) (OtherActor :type Actor%20Object%20Reference) (OtherComp :type Primitive%20Component%20Object%20Reference) (OtherBodyIndex :type Integer) (bFromSweep :type Boolean) (SweepResult :type Hit%20Result%20Structure%20%28by%20ref%29))
  (Utilities|Casting|CastToI_PlayerSideDamageable OtherActor)
  (CallFunction|DeadServer))

(event Custom|Move
  (bind _point (Default|ImpactPoint (Variables|Default|GetTarget)))
  (bind _output_get (Variables|Default|SetStartMovementPoint (Transformation|GetActorLocation)))
  (Variables|Default|SetEndMovementPoint (+ _output_get (* (Math|Vector|Normalize (- _point _output_get) 0.1) (Variables|Default|GetSpeed))))
  (bind _alpha (Timeline|TL_Move PlayFromStart)
    (:Update
      (Transformation|SetActorLocation (Math|Vector|Lerp(Vector) (Variables|Default|GetStartMovementPoint) (Variables|Default|GetEndMovementPoint) _alpha) false false))))

(event Custom|Explode
  (Game|SpawnActorfromClass "/Game/Blueprints/Damageable/BP_Explosion.BP_Explosion_C" (Math|Transform|MakeTransform (Transformation|GetActorLocation) "0, 0, 0" "1.000000,1.000000,1.000000") "AlwaysSpawn" "MultiplyWithRoot" 0 1.2e+02 1e+01 self true 0))

(event EventBeginPlay
  (|CallParentFunction)
  (Components|Timeline|SetPlayRate (Variables|Default|GetTL_Move) (/ 1.0 (Variables|Default|GetMovementTime)))
  (Utilities|Time|SetTimerbyEvent (delegate Custom|Move) (Variables|Default|GetMovementTime) true false 2.0))

(event Collision|EventActorBeginOverlap
  (params (OtherActor :type Actor%20Object%20Reference)))

(event EventTick
  (params (DeltaSeconds :type Float%20%28single-precision%29)))

(event EventDeadLocal
  (CallFunction|Explode)
  (Actor|DestroyActor))

(fn ConstructionScript
  (|CallParentFunction)
  (Variables|Default|SetMoveCooldown -1.0)
  (Variables|Default|SetAttackCooldown -1.0)
  (Variables|Default|SetTimeMoving -1.0)
  (Variables|Default|SetTimeToRecalculateTarget 2.0))

(fn SetDiffLevel
  (params (DifLevel :type Integer))
  (|CallParentFunction DifLevel)
  (Variables|Default|SetSpeed (Utilities|Select :Index DifLevel :Option%200 5e+01 :Option%201 75.0 :Option%202 1e+02 :Option%203 125.0 :Option%204 1.5e+02)))