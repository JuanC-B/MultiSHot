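; BP_BomberProjectile is a projectile that explodes on overlap, ignoring BP_NE_Bombs enemies and other bomber projectiles.
; On BeginPlay, a Server, Cast and Local event chain applies its Velocity variable to the ProjectileMovement component.
; A DoOnce on the Sphere overlap resets for ignored actors; otherwise the projectile spawns a damaging BP_Explosion and destroys itself.
; Static mesh hits only print a debug string.
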(event OnComponentHit(StaticMesh)
  (params (HitComponent :type Primitive%20Component%20Object%20Reference) (OtherActor :type Actor%20Object%20Reference) (OtherComp :type Primitive%20Component%20Object%20Reference) (NormalImpulse :type Vector :default "0, 0, 0") (Hit :type Hit%20Result%20Structure%20%28by%20ref%29))
  (Development|PrintString "HITHITHITHITHITHITHITHITHITHIT" true true "(R=1.000000,G=0.000000,B=0.336177,A=1.000000)"))

(event OnComponentBeginOverlap(Sphere)
  (params (OverlappedComponent :type Primitive%20Component%20Object%20Reference) (OtherActor :type Actor%20Object%20Reference) (OtherComp :type Primitive%20Component%20Object%20Reference) (OtherBodyIndex :type Integer) (bFromSweep :type Boolean) (SweepResult :type Hit%20Result%20Structure%20%28by%20ref%29))
  (Utilities|FlowControl|DoOnce false :!label _label
    (:Completed
      (Utilities|Casting|CastToBP_NE_Bombs OtherActor
        (:then
          (goto _label Reset))
        (:CastFailed
          (Utilities|Casting|CastToBP_BomberProjectile OtherActor
            (:then
              (goto _label Reset))
            (:CastFailed
              (CallFunction|Explode)
              (Actor|DestroyActor))))))))

(event Custom|Local_Launch
  (bind _projectilemovement (Variables|Default|GetProjectileMovement))
  (bind _output_get (Variables|/Script/Engine.MovementComponent|SetVelocity _projectilemovement (Variables|Default|GetVelocity)))
  (Variables|/Script/Engine.ProjectileMovementComponent|SetInitialSpeed _projectilemovement (Math|Vector|VectorLength _output_get)))

(event Custom|Explode
  (Game|SpawnActorfromClass "/Game/Blueprints/Damageable/BP_Explosion.BP_Explosion_C" (Math|Transform|MakeTransform (Transformation|GetActorLocation) "0, 0, 0" "1.000000,1.000000,1.000000") "AlwaysSpawn" "MultiplyWithRoot" 0 9e+01 5.0 self true 0))

(event Custom|Cast_Launch
  (CallFunction|LocalLaunch))

(event Custom|Server_Launch
  (CallFunction|CastLaunch))

(event EventBeginPlay
  (CallFunction|ServerLaunch))

(fn ConstructionScript)