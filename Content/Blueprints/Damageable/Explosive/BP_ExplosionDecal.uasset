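; Explosion decal actor that shows a mesh scorch mark with animated glow and opacity, then destroys itself.
; BeginPlay passes a random bool through a server, replicate and local event chain to pick one of two decal materials.
; A slowed timeline then drives emissive and opacity parameters on a dynamic material instance, and the actor is destroyed when it finishes.
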(event Custom|ReplicateBeginplay
  (params (Index :type Boolean))
  (CallFunction|LocalBegin Index))

(event Custom|LocalBegin
  (params (Index :type Boolean))
  (Rendering|Material|SetMaterial (Variables|Default|GetStaticMesh) 0 (select Index "/Game/VFX/MI_MEshDecalExplosion2.MI_MEshDecalExplosion2" "/Game/VFX/MI_MEshDecalExplosion.MI_MEshDecalExplosion")))

(event Custom|BeginServer
  (params (Index :type Boolean))
  (CallFunction|ReplicateBeginplay Index))

(event EventBeginPlay
  (CallFunction|BeginServer (Math|Random|RandomBool))
  (Components|Timeline|SetPlayRate (Variables|Default|GetTL_emissionDecay) 0.25)
  (bind _returnvalue (Rendering|Material|CreateDynamicMaterialInstance (Variables|Default|GetStaticMesh) 0 0 "None" :!class /Script/Engine.PrimitiveComponent))
  (Variables|Default|SetMaterialRef _returnvalue)
  (bind (_direction _alpha _fade) (Timeline|TL_emissionDecay Play)
    (:Update
      (Rendering|Material|SetScalarParameterValue (Variables|Default|GetMaterialRef) "Emissive Value" (Math|Float|Lerp 0.0 1e+01 _alpha) :!class /Script/Engine.MaterialInstanceDynamic)
      (Rendering|Material|SetScalarParameterValue (Variables|Default|GetMaterialRef) "Opacity Intensity" (Math|Float|Lerp 1.0 0.0 _fade) :!class /Script/Engine.MaterialInstanceDynamic))
    (:Finished
      (Actor|DestroyActor))))

(event Collision|EventActorBeginOverlap
  (params (OtherActor :type Actor%20Object%20Reference)))

(event EventTick
  (params (DeltaSeconds :type Float%20%28single-precision%29)))

(fn ConstructionScript)