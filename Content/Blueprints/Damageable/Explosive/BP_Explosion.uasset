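; Explosion actor that deals silent damage through I_Damageable to everything inside its radius sphere, except the ignored instigator.
; BeginPlay passes a random pitch through a server/replication event chain that sets effect visibility and Niagara size variant; the radius-based sound is unconnected.
; After a brief delay it spawns a distance-scaled floor decal, then applies damage.
; It destroys itself a second later only if something overlapped.
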(event Custom|ReplicateBeginplay
  (params (A :type Float%20%28double-precision%29))
  (CallFunction|LocalBegin A))

(event Custom|LocalBegin
  (params (A :type Float%20%28double-precision%29))
  (bind _showparticle (Variables|Default|GetShowParticle))
  (Development|SetHiddeninGame (Variables|Default|GetNiagara) (not _showparticle) false)
  (Development|SetHiddeninGame (Variables|Default|GetSphere) _showparticle false)
  (if (>= (Variables|Default|GetRadious) 75.0)
    (Class|NiagaraComponent|SetAsset (Variables|Default|GetNiagara) "/Game/VFX/NS_Explosion_B.NS_Explosion_B" true)))

(event Custom|BeginServer
  (params (A :type Float%20%28double-precision%29))
  (CallFunction|ReplicateBeginplay A))

(event EventBeginPlay
  (bind _returnvalue (Transformation|GetActorLocation))
  (bind _floorz (Variables|Default|GetFloorZ))
  (bind _sphere (Variables|Default|GetSphere))
  (bind (_x _y _z) (Math|Vector|BreakVector _returnvalue))
  (bind _overlappingactors (Collision|GetOverlappingActors _sphere 0 :!class /Script/Engine.PrimitiveComponent))
  (CallFunction|BeginServer (Math|Random|RandomFloatinRange 0.8 1.1))
  (Utilities|FlowControl|Delay 0.05)
  (Utilities|FlowControl|Sequence
    (:then_0
      (if (Variables|Default|GetShowParticle)
        (Variables|Default|SetBombDistance (- _floorz (- _z (Variables|Default|GetRadious))))
        (if (>= (Variables|Default|GetBombDistance) 0.0)
          (Game|SpawnActorfromClass "/Game/Blueprints/Damageable/Explosive/BP_ExplosionDecal.BP_ExplosionDecal_C" (Math|Transform|MakeTransform (Math|Vector|MakeVector _x _y _floorz) (Math|Rotator|MakeRotator 0.0 0.0 (Math|Random|RandomFloatinRange 0.0 359.0)) (Math|Vector|MakeVector (Math|Float|MapRangeClamped (Variables|Default|GetBombDistance) 0.0 1e+02 0.2 2.0) (Math|Float|MapRangeClamped (Variables|Default|GetBombDistance) 0.0 1e+02 0.2 2.0) (Math|Float|MapRangeClamped (Variables|Default|GetBombDistance) 0.0 1e+02 0.2 2.0))) "AlwaysSpawn" "MultiplyWithRoot" 0 0))))
    (:then_1
      (Components|Sphere|SetSphereRadius _sphere (Variables|Default|GetRadious) true)
      (if (>= (Utilities|Array|Length _overlappingactors) 1)
        (bind _output_get (Variables|Default|SetLastIndex (Utilities|Array|LastIndex _overlappingactors)))
        (for _index (range 0 _output_get)
          (bind _asi_damageable (Utilities|Casting|CastToI_Damageable (Utilities|Array|Get(acopy) _overlappingactors _index)))
          (if (and (!= (Utilities|Array|Get(acopy) _overlappingactors _index) (Variables|Default|GetInstigatorToIgnore)) (Utilities|IsValid (Utilities|Array|Get(acopy) _overlappingactors _index)))
            (Default|SilentDamage _asi_damageable (Variables|Default|GetDamage))))
        (Utilities|FlowControl|Delay 1.0)
        (Actor|DestroyActor)))))

(fn ConstructionScript
  (bind _showparticle (Variables|Default|GetShowParticle))
  (Components|Activation|SetAutoActivate (Variables|Default|GetNiagara) _showparticle)
  (Development|SetHiddeninGame (Variables|Default|GetSphere) _showparticle false))