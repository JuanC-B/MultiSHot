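; BP_WM_RocketWeapon is a rocket weapon that fires BP_Rocket projectiles.
; It overrides ShotWeaponLocal, calling the parent logic and then spawning a rocket at the FirePoint transform.
; The new rocket receives OutHitLocation as its objective position through ShotRocket.
; BeginPlay, overlap and Tick are disabled stubs, and the construction script only calls its parent.
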(event EventBeginPlay
  (|CallParentFunction) ; This node is disabled and will not be called.\nDrag off pins to build functionality.
)

(event Collision|EventActorBeginOverlap
  (params (OtherActor :type Actor%20Object%20Reference)))

(event EventTick
  (params (DeltaSeconds :type Float%20%28single-precision%29))
  (|CallParentFunction DeltaSeconds) ; This node is disabled and will not be called.\nDrag off pins to build functionality.
)

(event EventShotWeaponLocal
  (|CallParentFunction)
  (bind _returnvalue (Game|SpawnActorfromClass "/Game/Blueprints/Weapons/Rocket_Weapon/BP_Rocket.BP_Rocket_C" (Transformation|GetWorldTransform (Variables|Default|GetFirePoint)) "Undefined" "MultiplyWithRoot" 0 0))
  (Default|ShotRocket _returnvalue 0 (Variables|Default|GetOut%20Hit%20Location)))

(fn ConstructionScript
  (|CallParentFunction))