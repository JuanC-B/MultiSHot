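; Rocket projectile that flies from its spawn point to a target position with a smoke trail, then explodes.
; A timeline lerps the mesh along the path, and the first overlap or the timeline's end spawns BP_Explosion and destroys the rocket.
; Rarity sets flight time and damage.
; Shot and explosion run locally at once, while Server-to-Cast event chains replay them for players not locally controlled.
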(event OnComponentBeginOverlap(Collision)
  (params (OverlappedComponent :type Primitive%20Component%20Object%20Reference) (OtherActor :type Actor%20Object%20Reference) (OtherComp :type Primitive%20Component%20Object%20Reference) (OtherBodyIndex :type Integer) (bFromSweep :type Boolean) (SweepResult :type Hit%20Result%20Structure%20%28by%20ref%29))
  (Utilities|FlowControl|DoOnce false
    (:Completed
      (Development|PrintString (Utilities|String|Append (Utilities|GetDisplayName OtherActor) (Utilities|GetDisplayName OtherComp)))
      (CallFunction|Explosion))))

(event Custom|ShotRocket
  (params (Player :type Character%20Object%20Reference) (ShootDirection :type Vector))
  (Variables|Default|SetPlayer Player)
  (CallFunction|ShotRocketServer Player ShootDirection)
  (CallFunction|ShotRocketLocal ShootDirection))

(event Custom|ShotRocketServer
  (params (Player :type Character%20Object%20Reference) (Objective%20Position :type Vector))
  (CallFunction|ShotRocketCast Player Objective%20Position))

(event Custom|ShotRocketCast
  (params (Player :type Character%20Object%20Reference) (Objective%20Position :type Vector))
  (if (not (Pawn|IsLocallyControlled Player))
    (CallFunction|ShotRocketLocal Objective%20Position)))

(event Custom|ShotRocketLocal
  (params (Objective%20Position :type Vector))
  (Components|Timeline|SetPlayRate (Variables|Default|GetRoad) (/ 1.0 (Utilities|Select :Index (Variables|Default|GetRare) :NewEnumerator0 1.25 :NewEnumerator1 1.0 :NewEnumerator2 0.75 :NewEnumerator3 0.5)))
  (bind _shot (Timeline|Road PlayFromStart)
    (:Update
      (Transformation|SetWorldLocation (Variables|Debug|GetStaticMeshComponent) (Math|Vector|Lerp(Vector) (Variables|Default|GetShot%20Start) Objective%20Position _shot) false false))
    (:Finished
      (CallFunction|Explosion))))

(event Custom|Explosion
  (CallFunction|ExplosionServer)
  (CallFunction|ExplosionLocal))

(event Custom|ExplosionServer
  (CallFunction|ExplosionCast))

(event Custom|ExplosionCast
  (bind _ascharacter (Utilities|Casting|CastToCharacter (Variables|Default|GetPlayer)))
  (if (not (Pawn|IsLocallyControlled _ascharacter))
    (CallFunction|ExplosionLocal)))

(event Custom|ExplosionLocal
  (Game|SpawnActorfromClass "/Game/Blueprints/Damageable/Explosive/BP_Explosion.BP_Explosion_C" (Math|Transform|MakeTransform (Transformation|GetWorldLocation (Variables|Default|GetBullet)) "0, 0, 0" "1.000000,1.000000,1.000000") "Undefined" "MultiplyWithRoot" 0 8e+01 (Utilities|Select :Index (Variables|Default|GetRare) :NewEnumerator0 2e+01 :NewEnumerator1 25.0 :NewEnumerator2 3e+01 :NewEnumerator3 3e+01) self true 0)
  (Actor|DestroyActor))

(event EventBeginPlay
  (bind _vfxspawn (Variables|Default|GetVFXSpawn))
  (Variables|Default|SetShot%20Start (Transformation|GetWorldLocation (Variables|Default|GetBullet)))
  (Effects|SpawnEmitterAttached (Variables|Default|GetVFXSmokeTrail) _vfxspawn "None" (Transformation|GetWorldLocation _vfxspawn)))

(fn ConstructionScript)