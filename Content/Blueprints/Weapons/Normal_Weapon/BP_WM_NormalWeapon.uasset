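; Standard hitscan weapon for the VR character, extending a parent weapon's local shot and ray-tracing from an Arrow component.
; Non-player-side damageables take damage credited to the owning character, while non-damageable hits spawn a normal-aligned bullet decal; every hit type spawns impact VFX.
; Shots, except on player-side damageables, increase a capped deviation that raises the trace endpoint and widens its random Y offset until ResetShot clears it.
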(event EventBeginPlay
  (|CallParentFunction) ; This node is disabled and will not be called.\nDrag off pins to build functionality.
)

(event Collision|EventActorBeginOverlap
  (params (OtherActor :type Actor%20Object%20Reference)))

(event EventTick
  (params (DeltaSeconds :type Float%20%28single-precision%29))
  (|CallParentFunction DeltaSeconds) ; This node is disabled and will not be called.\nDrag off pins to build functionality.
)

(event EventShotWeaponLocal
  (bind _bulletsize (Variables|Default|GetbulletSize))
  (bind _arrow (Variables|Default|GetArrow))
  (bind _distancia_mira (Variables|Default|GetDistancia%20Mira))
  (bind _returnvalue (Math|Vector|GetForwardVector _arrow))
  (bind _returnvalue_2 (Transformation|GetWorldLocation _arrow))
  (bind _returnvalue_3 (* _returnvalue _distancia_mira))
  (bind _returnvalue_4 (+ _returnvalue_2 _returnvalue_3))
  (bind (_x _y _z) (Math|Vector|BreakVector _returnvalue_4))
  (|CallParentFunction)
  (bind _outhit (Collision|LineTraceByChannel _returnvalue_2 (Math|Vector|MakeVector _x (+ _y (/ (Math|Random|RandomFloatinRange (Variables|Default|GetDesvio%20Arma) (* (Variables|Default|GetDesvio%20Arma) -1.0)) 2.0)) (+ _z (Variables|Default|GetDesvio%20Arma))) "TraceTypeQuery2" false 0 "None" true "(R=1.000000,G=0.000000,B=0.000000,A=1.000000)" "(R=0.000000,G=1.000000,B=0.000000,A=1.000000)" 0.2))
  (if (Utilities|DoesObjectImplementInterface (.hitactor _outhit) "/Game/Blueprints/Damageable/I_Damageable.I_Damageable_C")
    (if (Utilities|DoesObjectImplementInterface (.hitactor _outhit) "/Game/Blueprints/Damageable/I_PlayerSideDamageable.I_PlayerSideDamageable_C")
      (Niagara|SpawnSystematLocation (Variables|Default|GetBulletHitVFX) (+ (.impactpoint _outhit) (.normal _outhit)) "0, 0, 0" (Variables|Default|GetVFXHitScale))
      (else
        (bind _asbp_vrcharacter__ (Utilities|Casting|CastToBP_VRCharacter__ (Components|GetOwner)))
        (Class|IDamageable|TryDamage(Message) (.hitactor _outhit) (Variables|Default|GetWeapon%20Values%20Damage) (.impactpoint _outhit) _asbp_vrcharacter__)
        (Niagara|SpawnSystematLocation (Variables|Default|GetBulletHitVFX) (.impactpoint _outhit) "0, 0, 0" (Variables|Default|GetVFXHitScale))
        (if (not (>= (+ (Variables|Default|GetDesvio%20Arma) (Variables|Default|GetWeapon%20Values%20Weapon%20Dispersion)) 9e+01))
          (Variables|Default|SetDesvio%20Arma (+ (Variables|Default|GetDesvio%20Arma) (Variables|Default|GetWeapon%20Values%20Weapon%20Dispersion))))))
    (else
      (Niagara|SpawnSystematLocation (Variables|Default|GetBulletHitVFX) (+ (.impactpoint _outhit) (.normal _outhit)) "0, 0, 0" (Variables|Default|GetVFXHitScale))
      (Game|SpawnActorfromClass "/Game/Blueprints/Weapons/SM_MeshDecal_Bullet.SM_MeshDecal_Bullet_C" (Math|Transform|MakeTransform (+ (.impactpoint _outhit) (.normal _outhit)) (Math|Rotator|MakeRotfromZX (.normal _outhit) (Math|Vector|RotateVectorAroundAxis (Transformation|GetActorForwardVector) (Class|KismetMathLibrary|DegAcos (Math|Vector|DotProduct (.normal _outhit) "0.000000,0.000000,1.000000")) (Math|Vector|Normalize (Math|Vector|CrossProduct (.normal _outhit) "0.000000,0.000000,1.000000")))) (Math|Vector|MakeVector _bulletsize _bulletsize _bulletsize)) "Undefined" "MultiplyWithRoot" 0 0)
      (if (not (>= (+ (Variables|Default|GetDesvio%20Arma) (Variables|Default|GetWeapon%20Values%20Weapon%20Dispersion)) 9e+01))
        (Variables|Default|SetDesvio%20Arma (+ (Variables|Default|GetDesvio%20Arma) (Variables|Default|GetWeapon%20Values%20Weapon%20Dispersion)))))))

(event EventResetShot
  (Variables|Default|SetDesvio%20Arma 0.0))

(fn ConstructionScript
  (|CallParentFunction))