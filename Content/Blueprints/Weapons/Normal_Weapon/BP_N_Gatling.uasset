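; Gatling gun weapon Blueprint that spins its barrel up while firing and winds it down on release.
; Fire input plays or reverses a timeline, slowed to one-third rate, that raises barrel rotation speed and shortens the shot cooldown, so fire rate ramps up with spin.
; Tick keeps rolling the barrel mesh at the current velocity, while parent calls handle the firing itself.
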(event Custom|OnTriggerInput
  (params (isPressed :type Boolean))
  (bind _sm_gatlingbarrel (Variables|Default|GetSM_GatlingBarrel))
  (if isPressed
    (bind _alpha (Timeline|TL_ShootSpeed Play)
      (:Update
        (Variables|Default|SetWeapon%20Values%20Shot%20Cooldown (Math|Float|Lerp 0.25 0.05 _alpha))
        (Variables|Default|SetRotationVelocity (Math|Float|Lerp 0.0 1e+01 _alpha))
        (Transformation|SetRelativeRotation _sm_gatlingbarrel (Math|Rotator|MakeRotator (+ (.Roll (Math|Rotator|BreakRotator (Variables|/Script/Engine.SceneComponent|GetRelativeRotation _sm_gatlingbarrel))) (Math|Float|Lerp 0.0 1e+01 _alpha)) 0.0 -89.999779) false false)))
    (else
      (Timeline|TL_ShootSpeed Reverse))))

(event EventBeginPlay
  (|CallParentFunction)
  (Components|Timeline|SetPlayRate (Variables|Default|GetTL_ShootSpeed) (/ 1.0 3.0)))

(event Collision|EventActorBeginOverlap
  (params (OtherActor :type Actor%20Object%20Reference))
  (|CallParentFunction OtherActor) ; This node is disabled and will not be called.\nDrag off pins to build functionality.
)

(event EventFireGunLocal
  (params (isShooting :type Boolean))
  (Utilities|FlowControl|Sequence
    (:then_0
      (CallFunction|OnTriggerInput isShooting))
    (:then_1
      (|CallParentFunction isShooting))))

(event EventTick
  (params (DeltaSeconds :type Float%20%28single-precision%29))
  (bind _sm_gatlingbarrel (Variables|Default|GetSM_GatlingBarrel))
  (|CallParentFunction DeltaSeconds)
  (Transformation|SetRelativeRotation _sm_gatlingbarrel (Math|Rotator|MakeRotator (+ (.Roll (Math|Rotator|BreakRotator (Variables|/Script/Engine.SceneComponent|GetRelativeRotation _sm_gatlingbarrel))) (Variables|Default|GetRotationVelocity)) 0.0 -89.999779) false false))

(fn ConstructionScript
  (|CallParentFunction))