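; Game instance that holds the player's Username and BestScore and persists them in the "GameData" save slot.
; LoadGame loads the existing SG_saveGame and copies its values into the instance, or creates a fresh save object when the slot is empty.
; SaveGame pushes both values into that object through SetVariablesThatNeedSave, then writes it to the slot asynchronously.
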(event Custom|SaveGame
  (bind _game_data_sg (Variables|Default|GetGame%20Data%20SG))
  (Default|SetVariablesThatNeedSave _game_data_sg (Variables|Default|GetUsername) (Variables|Default|GetBest%20Score))
  (|AsyncSaveGametoSlot _game_data_sg "GameData"))

(event Custom|LoadGame
  (bind _returnvalue (SaveGame|DoesSaveGameExist "GameData"))
  (if _returnvalue
    (bind _returnvalue_2 (SaveGame|LoadGamefromSlot "GameData"))
    (bind _assg_save_game (Utilities|Casting|CastToSG_saveGame _returnvalue_2))
    (Variables|Default|SetGame%20Data%20SG _assg_save_game)
    (CallFunction|LoadVariablesfromData)
    (else
      (bind _returnvalue_3 (SaveGame|CreateSaveGameObject "/Game/Blueprints/Data/SG_saveGame.SG_saveGame_C"))
      (Variables|Default|SetGame%20Data%20SG _returnvalue_3))))

(event Custom|LoadVariablesFromData
  (bind _game_data_sg (Variables|Default|GetGame%20Data%20SG))
  (Variables|Default|SetUsername (Variables|/Game/Blueprints/Data/SG_saveGame.SG_saveGame_C|GetUsername _game_data_sg))
  (Variables|Default|SetBest%20Score (Variables|/Game/Blueprints/Data/SG_saveGame.SG_saveGame_C|GetBestScore _game_data_sg)))