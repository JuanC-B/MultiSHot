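; BP_CON_Munition is a munition consumable that shows a colored robotic hand on its primary socket.
; Call_ShowSocket sets the hand texture by color index once, mirrors the socket scale for left or right, then makes it visible.
; Material, scale and visibility each pass through a Server, Cast and Local event chain, apparently for replication.
; A separate event also toggles socket visibility.
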(event Custom|Call_ShowSocket
  (params (IsLeft :type Boolean) (HandColorID :type Integer))
  (Utilities|FlowControl|Sequence
    (:then_0
      (|GetMaterialInstanceAndAssign_2 HandColorID))
    (:then_1
      (|CollapseGraph_2 IsLeft))
    (:then_2
      (|ShowHideHandsLogic_2))))

(event EventBeginPlay)

(event Collision|EventActorBeginOverlap
  (params (OtherActor :type Actor%20Object%20Reference)))

(event EventTick
  (params (DeltaSeconds :type Float%20%28single-precision%29)))

(fn ConstructionScript
  (|CallParentFunction))

(event Custom|Server_ManageHandMaterial
  (params (ColorIndex :type Integer))
  (CallFunction|CastManageHandMaterial ColorIndex))

(event Custom|Local_ManageHandMaterial
  (params (ColorIndex :type Integer))
  (bind _primarysocket_mesh (Variables|Default|GetPrimarySocket_Mesh))
  (Rendering|SetVisibility _primarysocket_mesh true false)
  (bind _returnvalue (Rendering|Material|CreateDynamicMaterialInstance _primarysocket_mesh 0 0 "None" :!class /Script/Engine.PrimitiveComponent))
  (Rendering|Material|SetTextureParameterValue _returnvalue "Base_color" (Utilities|Select :Index ColorIndex :Option%200 "/Game/VRHandsPack/Textures/T_Robotic_BC.T_Robotic_BC" :Option%201 "/Game/VRHandsPack/Textures/T_Robotic_BC_Green.T_Robotic_BC_Green" :Option%202 "/Game/VRHandsPack/Textures/T_Robotic_BC_Blue.T_Robotic_BC_Blue")))

(event Custom|Cast_ManageHandMaterial
  (params (ColorIndex :type Integer))
  (CallFunction|LocalManageHandMaterial ColorIndex))

(event Custom|Call_ShowHideShocket
  (params (NewVisibility :type Boolean))
  (CallFunction|ServerShowHideHand NewVisibility))

(event Custom|Server_ShowHideHand
  (params (NewVisibility :type Boolean))
  (CallFunction|CastShowHideHand NewVisibility))

(event Custom|Local_ShowHideHand
  (params (NewVisibility :type Boolean))
  (Rendering|SetVisibility (Variables|Default|GetPrimarySocket) NewVisibility true))

(event Custom|Cast_ShowHideHand
  (params (NewVisibility :type Boolean))
  (CallFunction|LocalShowHideHand NewVisibility))

(event Custom|Server_SetHandScale
  (params (isLeft :type Boolean))
  (CallFunction|CastSetHandScale isLeft))

(event Custom|Local_SetHandScale
  (params (isLeft :type Boolean))
  (Transformation|SetRelativeScale3D (Variables|Default|GetPrimarySocket) (select isLeft "-20.000000,20.000000,20.000000" "20.000000,20.000000,20.000000")))

(event Custom|Cast_SetHandScale
  (params (isLeft :type Boolean))
  (CallFunction|LocalSetHandScale isLeft))