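; BP_GST_Consumable is a consumable actor that destroys itself after a fixed cooldown from BeginPlay unless it has been picked up.
; Gripping it sets the Picked flag, which blocks the timed destruction, and enables overlap events on its static mesh.
; Both grip and destroy are relayed through Server, Cast and Local event chains, apparently to replicate them across the network.
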(event Custom|Server_Grip
  (CallFunction|CastGrip))

(event Custom|Cast_Grip
  (CallFunction|LocalGrip))

(event Custom|Local_Destroy
  ;[1 1 1] Destroy After Cooldown
  (Actor|DestroyActor))

(event Custom|Server_Destroy
  ;[1 1 1] Destroy After Cooldown
  (CallFunction|CastDestroy))

(event Custom|Cast_Destroy
  ;[1 1 1] Destroy After Cooldown
  (CallFunction|LocalDestroy))

(event Custom|DestroyAfterCooldown
  (params (Duration :type Float%20%28single-precision%29))
  ;[1 1 1] Destroy After Cooldown
  (Utilities|FlowControl|RetriggerableDelay Duration)
  (if (not (Variables|Default|GetPicked))
    (CallFunction|ServerDestroy)))

(event Custom|Local_Grip
  (Variables|Default|SetPicked true)
  (Variables|/Script/Engine.PrimitiveComponent|SetbGenerateOverlapEvents (Variables|Default|GetStaticMeshComponent) true))

(event EventBeginPlay
  (CallFunction|DestroyAfterCooldown 15.0))

(event EventOnGrip
  (params (GrippingController :type Grip%20Motion%20Controller%20Component%20Object%20Reference) (GripInformation :type BP%20Actor%20Grip%20Information%20Structure%20%28by%20ref%29))
  (CallFunction|ServerGrip))

(fn ConstructionScript)