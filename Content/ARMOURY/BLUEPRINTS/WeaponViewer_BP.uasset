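; Armoury weapon viewer actor that displays a swappable placeholder weapon and can serve as the player's view target.
; BeginPlay enables input, creates the weapon overlay widget and binds class-switch events that swap the WeaponActor child actor between handgun, machine gun and shotgun.
; SetCamera switches the player's view to this actor.
; Clicks and right or middle mouse buttons set rotate, move and displace flags, which this graph never reads.
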(event OnClicked(Cube)
  (params (TouchedComponent :type Primitive%20Component%20Object%20Reference) (ButtonPressed :type Key%20Structure :default "None"))
  (Variables|Default|SetCanRotate? true))

(event Custom|SetCamera
  (Game|Player|SetViewTargetwithBlend (Game|GetPlayerController 0) self 0.0 "VTBlend_Linear" 0.0 true))

(event Custom|SwitchClass_Shotgun
  ;[1 1 1] Placeholder for new upgrades
  (ChildActorComponent|SetChildActorClass (Variables|Default|GetWeaponActor) "/Game/ARMOURY/DEMO/BLUEPRINTS/Shotgun_Placeholder_BP.Shotgun_Placeholder_BP_C"))

(event Custom|SwitchClass_Handgun
  (ChildActorComponent|SetChildActorClass (Variables|Default|GetWeaponActor) "/Game/ARMOURY/DEMO/BLUEPRINTS/Handgun_Placeholder_BP.Handgun_Placeholder_BP_C"))

(event Custom|SwitchClass_MachineGun
  ;[1 1 1] Placeholder for new upgrades
  (ChildActorComponent|SetChildActorClass (Variables|Default|GetWeaponActor) "/Game/ARMOURY/DEMO/BLUEPRINTS/MachineGun_Placeholder_BP.MachineGun_Placeholder_BP_C"))

(event EventBeginPlay
  (Input|EnableInput (Game|GetPlayerController 0))
  (bind _returnvalue (UserInterface|CreateWidget "/Game/ARMOURY/BLUEPRINTS/UI/WeaponOverlay_WB.WeaponOverlay_WB_C"))
  (UserInterface|Viewport|AddtoViewport _returnvalue 0)
  (EventDispatchers|BindEventtoSwitchClassHandgun (delegate Custom|SwitchClass_Handgun))
  ;[1 1 1] Placeholder for new upgrades
  (EventDispatchers|BindEventtoSwitchClassMachineGun (delegate Custom|SwitchClass_MachineGun))
  (EventDispatchers|BindEventtoSwitchClassShotgun (delegate Custom|SwitchClass_Shotgun)))

(event MouseInput|EventActorOnClicked
  (params (ButtonPressed :type Key%20Structure :default "None"))
  (Variables|Default|SetCanRotate? true))

(event Input|MouseEvents|MiddleMouseButton
  (params (Key :type Key%20Structure :default "None"))
  (:Pressed
    (Variables|Default|SetCanDisplace? true))
  (:Released
    (Variables|Default|SetCanDisplace? false)))

(event Input|MouseEvents|RightMouseButton
  (params (Key :type Key%20Structure :default "None"))
  (:Pressed
    (Variables|Default|SetCanMove? true))
  (:Released
    (Variables|Default|SetCanMove? false)))

(fn ConstructionScript)