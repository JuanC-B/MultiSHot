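; Modular handgun actor that builds a randomised weapon variant on BeginPlay and through a bound Randomise event.
; Each roll writes random colours to Handgun_MPC, picks a Family, then swaps part meshes and toggles optional attachments, alternating the suppressor via FlipFlop.
; Substring checks on mesh and socket names gate magazine choice, canister and folding stock.
; A final pass applies shuffled Mat_List_DT materials matching mesh, slot and Family to visible main parts.
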(event Custom|Randomise_Event
  (bind _returnvalue (Math|Random|RandomFloat))
  (bind _returnvalue_2 (Math|Random|RandomFloat))
  (bind _returnvalue_3 (Math|Random|RandomFloat))
  (bind _returnvalue_4 (Math|Float|Clamp(Float) _returnvalue 0.3 0.8))
  (bind _returnvalue_5 (Math|Float|Clamp(Float) _returnvalue_2 0.3 0.8))
  (bind _returnvalue_6 (* _returnvalue_3 3.6e+02))
  (bind _returnvalue_7 (Math|Color|MakeColor _returnvalue_4 _returnvalue_4 _returnvalue_4))
  (Math|Float|CompareFloat (Math|Random|RandomFloat) 0.8
    (:>
      (Rendering|Material|SetVectorParameterValue "/Game/ARMOURY/Material_Layer_System/Handgun_MPC.Handgun_MPC" "Base_Color" (Class|KismetMathLibrary|HSVtoRGB _returnvalue_6 0.55 _returnvalue_5 1.0) :!class /Script/Engine.KismetMaterialLibrary :!label _label)
      (Rendering|Material|SetVectorParameterValue "/Game/ARMOURY/Material_Layer_System/Handgun_MPC.Handgun_MPC" "Base_Ceramic_Color" (Class|KismetMathLibrary|HSVtoRGB _returnvalue_6 0.8 1.0 1.0) :!class /Script/Engine.KismetMaterialLibrary))
    (:==
      (goto _label))
    (:<
      (Rendering|Material|SetVectorParameterValue "/Game/ARMOURY/Material_Layer_System/Handgun_MPC.Handgun_MPC" "Base_Color" _returnvalue_7 :!class /Script/Engine.KismetMaterialLibrary)
      (Rendering|Material|SetVectorParameterValue "/Game/ARMOURY/Material_Layer_System/Handgun_MPC.Handgun_MPC" "Base_Ceramic_Color" _returnvalue_7 :!class /Script/Engine.KismetMaterialLibrary)))
  (Rendering|Material|SetVectorParameterValue "/Game/ARMOURY/Material_Layer_System/Handgun_MPC.Handgun_MPC" "T_Flashlight_Color" (Class|KismetMathLibrary|HSVtoRGB (* (Math|Random|RandomFloat) 3.6e+02) 1.0 1.0 1.0) :!class /Script/Engine.KismetMaterialLibrary)
  (Rendering|Material|SetVectorParameterValue "/Game/ARMOURY/Material_Layer_System/Handgun_MPC.Handgun_MPC" "Accent_Color" (Class|KismetMathLibrary|HSVtoRGB (* (Math|Random|RandomFloat) 3.6e+02) 0.85 1.0 1.0) :!class /Script/Engine.KismetMaterialLibrary)
  (Rendering|Material|SetVectorParameterValue "/Game/ARMOURY/Material_Layer_System/Handgun_MPC.Handgun_MPC" "Floor_Color" (Class|KismetMathLibrary|HSVtoRGB (* (Math|Random|RandomFloat) 3.6e+02) 0.5 _returnvalue_5 1.0) :!class /Script/Engine.KismetMaterialLibrary)
  (Variables|Default|SetFamily (Math|Random|RandomInteger 3))
  (Utilities|FlowControl|Sequence
    (:then_0
      (CallFunction|GripSelectorEvent))
    (:then_1
      (CallFunction|BarrelSelectorEvent))
    (:then_2
      (CallFunction|MagSelectorEvent))
    (:then_3
      (CallFunction|SightSelectorEvent))
    (:then_4
      (CallFunction|SupressorSelectorEvent))
    (:then_5
      (CallFunction|FrontAddonEvent))
    (:then_6
      (CallFunction|FoldStockEvent))
    (:then_7
      (CallFunction|RandomizeMaterialEvent))))

(event Custom|Front_Addon_Event
  (bind _front_addons (Variables|Default|GetFront_Addons))
  ;[1 1 1] FRONT ADDON EVENT
  (Components|SkeletalMesh|SetSkeletalMeshAsset (Variables|Default|GetFront_Addons) (Utilities|Select :Index (Math|Random|RandomIntegerinRange 0 1) :Option%200 "/Game/ARMOURY/MESHES/HANDGUNS/ADDONS/FLASHLIGHT/Flashlight_01_SK.Flashlight_01_SK" :Option%201 "/Game/ARMOURY/MESHES/HANDGUNS/ADDONS/FGRIP/Fgrip_01_SK.Fgrip_01_SK"))
  (if (Math|Random|RandomBool)
    (Rendering|SetVisibility _front_addons true false)
    (else
      (Rendering|SetVisibility _front_addons false false))))

(event Custom|Randomize%20Material%20Event
  (bind _returnvalue (|GetandShuffleDataTableData))
  (for _array_element (Utilities|Array|MakeArray (Variables|Default|GetGrip) (Variables|Default|GetBarrel) (Variables|Default|GetFront_Addons) (Variables|Default|GetFoldStock))
    (if (Variables|/Script/Engine.SceneComponent|GetbVisible _array_element)
      (for _array_element_2 (Class|MeshComponent|GetMaterialSlotNames _array_element)
        (if (Math|Boolean|ANDBoolean (== (Variables|/Script/Engine.SkeletalMeshComponent|GetSkeletalMeshAsset _array_element) (.Mesh (Utilities|Struct|BreakMat_List_Struct _returnvalue))) (== (Rendering|Material|GetMaterialIndex _array_element _array_element_2) (.Index (Utilities|Struct|BreakMat_List_Struct _returnvalue))) (== (.Family (Utilities|Struct|BreakMat_List_Struct _returnvalue)) (Variables|Default|GetFamily)))
          (Rendering|Material|SetMaterial _array_element (.Index (Utilities|Struct|BreakMat_List_Struct _returnvalue)) (.Material_Instance (Utilities|Struct|BreakMat_List_Struct _returnvalue))))))))

(event Custom|Supressor_Selector_Event
  ;[1 1 1] SUPRESSOR SELECTOR
  (Utilities|FlowControl|FlipFlop
    (:A
      (Rendering|SetVisibility (Variables|Default|GetSuppressor) true false))
    (:B
      (Rendering|SetVisibility (Variables|Default|GetSuppressor) false false))))

(event Custom|Barrel_Selector_Event
  ;[1 1 1] BARREL
  (Components|SkeletalMesh|SetSkeletalMeshAsset (Variables|Default|GetBarrel) (Utilities|Select :Index (Math|Random|RandomIntegerinRange 0 3) :Option%200 "/Game/ARMOURY/MESHES/HANDGUNS/BARREL_01/Barrel_01_SK.Barrel_01_SK" :Option%201 "/Game/ARMOURY/MESHES/HANDGUNS/BARREL_02/Barrel_02_SK.Barrel_02_SK" :Option%202 "/Game/ARMOURY/MESHES/HANDGUNS/BARREL_03/Barrel_03_SK.Barrel_03_SK" :Option%203 "/Game/ARMOURY/MESHES/HANDGUNS/BARREL_04/Barrel_04_SK.Barrel_04_SK")))

(event Custom|Sight_Selector_Event
  (bind _picatinny (Variables|Default|GetPicatinny))
  ;[1 1 1] SIGHT SELECTOR
  (if (Math|Random|RandomBool)
    (Rendering|SetVisibility _picatinny true false)
    (Components|SkeletalMesh|SetSkeletalMeshAsset (Variables|Default|GetSight) (Utilities|Select :Index (Math|Random|RandomIntegerinRange 0 2) :Option%200 "/Game/ARMOURY/MESHES/HANDGUNS/SIGHT_01/Sight_01_SK.Sight_01_SK" :Option%201 "/Game/ARMOURY/MESHES/HANDGUNS/SIGHT_02/Sight_02_SK.Sight_02_SK" :Option%202 "/Game/ARMOURY/MESHES/HANDGUNS/SIGHT_03/Sight_03_SK.Sight_03_SK"))
    (Rendering|SetVisibility (Variables|Default|GetSight) (Math|Random|RandomBool) false)
    (else
      (Rendering|SetVisibility _picatinny false false)
      (Rendering|SetVisibility (Variables|Default|GetSight) false false))))

(event Custom|Grip_Selector_Event
  ;[1 1 1] GRIP SELECTOR
  (Components|SkeletalMesh|SetSkeletalMeshAsset (Variables|Default|GetGrip) (Utilities|Select :Index (Math|Random|RandomIntegerinRange 0 3) :Option%200 "/Game/ARMOURY/MESHES/HANDGUNS/GRIP_01/Grip_01_SK.Grip_01_SK" :Option%201 "/Game/ARMOURY/MESHES/HANDGUNS/GRIP_02/Grip_02_SK.Grip_02_SK" :Option%202 "/Game/ARMOURY/MESHES/HANDGUNS/GRIP_03/Grip_03_SK.Grip_03_SK" :Option%203 "/Game/ARMOURY/MESHES/HANDGUNS/GRIP_04/Grip_04_SK.Grip_04_SK")))

(event Custom|FoldStock_Event
  ;[1 1 1] FOLDSTOCK EVENT
  (for _array_element (Transformation|GetAllSocketNames (Variables|Default|GetBarrel))
    (if (Utilities|String|Contains (Utilities|String|ToString(Name) _array_element) "04")
      (Transformation|AttachComponentToComponent (Variables|Default|GetFoldStock) (Variables|Default|GetBarrel) _array_element "KeepRelative" "KeepRelative" "KeepRelative" true)
      (Rendering|SetVisibility (Variables|Default|GetFoldStock) (Math|Random|RandomBool) false)
      (else
        (Rendering|SetVisibility (Variables|Default|GetFoldStock) false false)))))

(event Custom|Mag_Selector_Event
  (bind _mags (Variables|Default|GetMags))
  ;[1 1 1] MAG SELECTOR
  (if (Utilities|String|Contains (Utilities|GetObjectName (Variables|/Script/Engine.SkeletalMeshComponent|GetSkeletalMeshAsset (Variables|Default|GetGrip))) "04")
    (Components|SkeletalMesh|SetSkeletalMeshAsset _mags (Utilities|Select :Index (Math|Random|RandomIntegerinRange 0 2) :Option%200 "/Game/ARMOURY/MESHES/HANDGUNS/MAG_02/Mag_02_SK.Mag_02_SK" :Option%201 "/Game/ARMOURY/MESHES/HANDGUNS/MAG_03/Mag_03_SK.Mag_03_SK" :Option%202 "/Game/ARMOURY/MESHES/HANDGUNS/MAG_04/Mag_04_SK.Mag_04_SK"))
    (else
      (Components|SkeletalMesh|SetSkeletalMeshAsset _mags (Utilities|Select :Index (Math|Random|RandomIntegerinRange 0 3) :Option%200 "/Game/ARMOURY/MESHES/HANDGUNS/MAG_01/Mag_01_SK.Mag_01_SK" :Option%201 "/Game/ARMOURY/MESHES/HANDGUNS/MAG_02/Mag_02_SK.Mag_02_SK" :Option%202 "/Game/ARMOURY/MESHES/HANDGUNS/MAG_03/Mag_03_SK.Mag_03_SK" :Option%203 "/Game/ARMOURY/MESHES/HANDGUNS/MAG_04/Mag_04_SK.Mag_04_SK"))))
  (if (Utilities|String|Contains (Utilities|GetObjectName (Variables|/Script/Engine.SkeletalMeshComponent|GetSkeletalMeshAsset (Variables|Default|GetMags))) "04")
    (Transformation|AttachComponentToComponent (Variables|Default|GetSub_Addon) (Variables|Default|GetMags) "Cannister_Socket" "KeepRelative" "KeepRelative" "KeepRelative" true)
    (Rendering|SetVisibility (Variables|Default|GetSub_Addon) (Math|Random|RandomBool) false)
    (else
      (Rendering|SetVisibility (Variables|Default|GetSub_Addon) false false))))

(event EventBeginPlay
  (Variables|Default|SetHandgun_Set (Utilities|Array|MakeArray (Variables|Default|GetGrip) (Variables|Default|GetBarrel) (Variables|Default|GetMags) (Variables|Default|GetSub_Addon) (Variables|Default|GetPicatinny) (Variables|Default|GetSuppressor) (Variables|Default|GetFront_Addons) (Variables|Default|GetFoldStock) (Variables|Default|GetSight)))
  (EventDispatchers|BindEventtoRandomise (delegate Custom|Randomise_Event))
  (CallFunction|RandomiseEvent))

(event Collision|EventActorBeginOverlap
  (params (OtherActor :type Actor%20Object%20Reference)))

(event EventTick
  (params (DeltaSeconds :type Float%20%28single-precision%29)))

(fn ConstructionScript)